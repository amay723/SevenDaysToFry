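; Onion ingredient spawner that hands the player a fresh onion when interacted with.
; Interact spawns BP_Ingredient_Onions just above the spawner, attaches it to player character 0 keeping its world transform, and disables its collision.
; While InteractArrow is visible, Tick plays a self-restarting timeline that adds its track value to the arrow's current relative Z to animate it.
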(event EventBeginPlay)

(event Collision|EventActorBeginOverlap
  (params (OtherActor :type Actor%20Object%20Reference)))

(event EventTick
  (params (DeltaSeconds :type Float%20%28single-precision%29))
  (bind _interactarrow (Variables|Default|GetInteractArrow))
  (if (Rendering|IsVisible _interactarrow)
    (bind _newtrack_1 (Timeline|Timeline_0 Play)
      (:Update
        (Transformation|SetRelativeLocation _interactarrow (Math|Vector|MakeVector 0.0 0.0 (+ (.x _newtrack_1) (.z (Variables|/Script/Engine.SceneComponent|GetRelativeLocation _interactarrow)))) false false))
      (:Finished
        (if true
          (Timeline|Timeline_0 PlayFromStart))))))

(event EventInteract
  (bind _returnvalue (Transformation|GetActorTransform))
  (bind _returnvalue_2 (Game|SpawnActorfromClass "/Game/RecipeData/Ingredients/BP_Ingredient_Onions.BP_Ingredient_Onions_C" (Math|Transform|MakeTransform (Math|Vector|MakeVector (.x (.location _returnvalue)) (.y (.location _returnvalue)) (+ (.z (.location _returnvalue)) 35.0)) (.rotation _returnvalue) (.scale _returnvalue)) "Undefined" 0 0))
  (bind _output_get (Variables|Default|SetBP_Ingredient_Onions_Instance _returnvalue_2))
  (Transformation|AttachActorToActor _returnvalue_2 (Game|GetPlayerCharacter 0) "None" "KeepWorld" "KeepWorld" "KeepWorld" true)
  (Collision|SetActorEnableCollision _output_get false))

(fn ConstructionScript)