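; Grill station that cooks a patty the player places on it through Interact.
; Interacting while holding "Patty" spawns a grilled patty actor on top, and Tick then advances a camera-facing progress bar widget toward a hard-coded cook threshold.
; Once cooked, an empty-handed Interact replaces that actor with a fresh one attached to the player, collision disabled.
; A looping timeline bobs the interact arrow while visible.
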(event EventBeginPlay
  ;[1 1 1] Begin Play
  (bind _asbp_grill_progress_bar (Utilities|Casting|CastToBP_Grill_Progress_Bar (UserInterface|GetUserWidgetObject (Variables|Default|GetGrillProgressBar))))
  (Variables|Default|SetBP_Grill_Progress_Bar _asbp_grill_progress_bar)
  (bind _output_get (Variables|/Game/FinalProjectBlueprints/BP_Grill_Progress_Bar.BP_Grill_Progress_Bar_C|SetGrillingProgress (Variables|Default|GetBP_Grill_Progress_Bar) 0.0))
  (Variables|/Game/FinalProjectBlueprints/BP_Grill_Progress_Bar.BP_Grill_Progress_Bar_C|SetTimeToGrill (Variables|Default|GetBP_Grill_Progress_Bar) 8.0)
  (Default|UpdateGrillingProgress (Variables|Default|GetBP_Grill_Progress_Bar) _output_get)
  (Widget|SetVisibility (Variables|Default|GetBP_Grill_Progress_Bar) "Hidden"))

(event Collision|EventActorBeginOverlap
  (params (OtherActor :type Actor%20Object%20Reference)))

(event EventTick
  (params (DeltaSeconds :type Float%20%28single-precision%29))
  (bind _interactarrow (Variables|Default|GetInteractArrow))
  (Utilities|FlowControl|Sequence
    (:then_0
      ;[1 1 1] Interact Arrow
      (if (Rendering|IsVisible _interactarrow)
        (bind _newtrack_1 (Timeline|Timeline_0 Play)
          (:Update
            (Transformation|SetRelativeLocation _interactarrow (Math|Vector|MakeVector 0.0 0.0 (+ (.x _newtrack_1) (.z (Variables|/Script/Engine.SceneComponent|GetRelativeLocation _interactarrow)))) false false))
          (:Finished
            (if true
              (Timeline|Timeline_0 PlayFromStart))))))
    (:then_1
      ;[1 1 1] Progress Bar
      (CallFunction|RotateGrillingProgressBartoPlayer)
      (if (Variables|Default|GetIsPattyOnGrill)
        (Widget|SetVisibility (Variables|Default|GetBP_Grill_Progress_Bar) "Visible")
        (CallFunction|ModifyGrillingProgress DeltaSeconds)
        (Default|UpdateGrillingProgress (Variables|Default|GetBP_Grill_Progress_Bar) (Variables|Default|GetGrillingProgress))
        (if (>= (Variables|Default|GetGrillingProgress) 8.0)
          (Variables|Default|SetIsPattyCooked true))
        (elif (!= (Variables|Default|GetGrillingProgress) 0.0)
          (Variables|Default|SetGrillingProgress 0.0)
          (Widget|SetVisibility (Variables|Default|GetBP_Grill_Progress_Bar) "Hidden"))))))

(event EventInteract
  (bind _returnvalue (Transformation|GetActorLocation))
  (bind _asbp_character (Utilities|Casting|CastToBP_Character (Game|GetPlayerCharacter 0)))
  (if (Variables|Default|GetIsPattyOnGrill)
    (if (Utilities|Enum|Equal(Enum) (Variables|/Game/FinalProjectBlueprints/BP_Character.BP_Character_C|GetIngredientHeldByPlayer _asbp_character) "None")
      (if (Variables|Default|GetIsPattyCooked)
        (Actor|DestroyActor (stale _returnvalue_3))
        (Variables|Default|SetIsPattyOnGrill false)
        (bind _returnvalue_2 (Game|SpawnActorfromClass "/Game/RecipeData/Ingredients/BP_Ingredient_Grilled_Patty.BP_Ingredient_Grilled_Patty_C" (Variables|Default|GetPattyOnGrillTransform) "Undefined" 0 0))
        (bind _output_get (Variables|Default|SetBP_Ingredient_Grilled_Patty_Instance _returnvalue_2))
        (Transformation|AttachActorToActor _output_get (Game|GetPlayerCharacter 0) "None" "KeepWorld" "KeepWorld" "KeepWorld" true)
        (Collision|SetActorEnableCollision _output_get false)))
    (elif (Utilities|Enum|Equal(Enum) (Variables|/Game/FinalProjectBlueprints/BP_Character.BP_Character_C|GetIngredientHeldByPlayer _asbp_character) "Patty")
      (bind _returnvalue_3 (Game|SpawnActorfromClass "/Game/RecipeData/Ingredients/BP_Ingredient_Grilled_Patty.BP_Ingredient_Grilled_Patty_C" (Math|Transform|MakeTransform (Math|Vector|MakeVector (.x _returnvalue) (.y _returnvalue) (+ (.z _returnvalue) 115.0)) "0, 0, 0" "1,1,1") "Undefined" 0 0))
      (Variables|Default|SetIsPattyOnGrill true)
      (Variables|Default|SetPattyOnGrillTransform (Transformation|GetActorTransform _returnvalue_3)))))

(fn ConstructionScript)

(fn ModifyGrillingProgress
  (params (TimeToAdd :type Float%20%28single-precision%29))
  (Variables|Default|SetGrillingProgress (Math|Float|Clamp(Float) (+ TimeToAdd (Variables|Default|GetGrillingProgress)) 0.0 (Variables|Default|GetTimeToGrill))))

(fn RotateGrillingProgressBartoPlayer
  (Transformation|SetWorldRotation (Variables|Default|GetGrillProgressBar) (Math|Rotator|FindLookatRotation (Transformation|GetWorldLocation (Variables|Default|GetGrillProgressBar)) (Camera|GetCameraLocation (Game|GetPlayerCameraManager 0))) false false)
  (return))