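; Counter slot that assembles a finished burger from ingredients on two other counter slots when interacted with.
; Interact reads both slot instances and the current order from BP_Character, then sets bun and grilled patty flags from each slot's ingredient name.
; For a Burger order with both flags set, it destroys the ingredient actors, resets the slots to None and spawns BP_Burger above itself, keeping a reference.
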(event EventBeginPlay)

(event Collision|EventActorBeginOverlap
  (params (OtherActor :type Actor%20Object%20Reference)))

(event EventTick
  (params (DeltaSeconds :type Float%20%28single-precision%29)))

(event EventInteract
  (bind _returnvalue (Transformation|GetActorLocation))
  (bind _asbp_character (Utilities|Casting|CastToBP_Character (Game|GetPlayerCharacter 0)))
  (bind _output_get (Variables|Default|SetBP_Counter_Slot_1 (Variables|/Game/FinalProjectBlueprints/BP_Character.BP_Character_C|GetBP_Counter_Slot_1_Instance _asbp_character)))
  (bind _output_get_2 (Variables|Default|SetBP_Counter_Slot_2 (Variables|/Game/FinalProjectBlueprints/BP_Character.BP_Character_C|GetBP_Counter_Slot_2_Instance _asbp_character)))
  (Variables|Default|SetCurrentOrder (Variables|/Game/FinalProjectBlueprints/BP_Character.BP_Character_C|GetCurrentOrder _asbp_character))
  (Utilities|FlowControl|Sequence
    (:then_0
      (if (Utilities|Enum|Equal(Enum) (Variables|/Game/FinalProjectBlueprints/BP_Counter_slot_1.BP_Counter_Slot_1_C|GetIngredientOnCounterSlot1 _output_get) "Buns")
        (Variables|Default|SetIsBunsPresent true)
        (elif (Utilities|Enum|Equal(Enum) (Variables|/Game/FinalProjectBlueprints/BP_Counter_slot_1.BP_Counter_Slot_1_C|GetIngredientOnCounterSlot1 _output_get) "GrilledPatty")
          (Variables|Default|SetIsGrilledPattyPresent true)
          (elif (Utilities|Enum|Equal(Enum) (Variables|/Game/FinalProjectBlueprints/BP_Counter_slot_1.BP_Counter_Slot_1_C|GetIngredientOnCounterSlot1 _output_get) "None")
            (Variables|Default|SetIsBunsPresent false)
            (Variables|Default|SetIsGrilledPattyPresent false)))))
    (:then_1
      (if (Utilities|Enum|Equal(Enum) (Variables|/Game/FinalProjectBlueprints/BP_Counter_Slot_2.BP_Counter_Slot_2_C|GetIngredientOnCounterSlot2 _output_get_2) "Buns")
        (Variables|Default|SetIsBunsPresent true)
        (elif (Utilities|Enum|Equal(Enum) (Variables|/Game/FinalProjectBlueprints/BP_Counter_Slot_2.BP_Counter_Slot_2_C|GetIngredientOnCounterSlot2 _output_get_2) "GrilledPatty")
          (Variables|Default|SetIsGrilledPattyPresent true)
          (elif (Utilities|Enum|Equal(Enum) (Variables|/Game/FinalProjectBlueprints/BP_Counter_Slot_2.BP_Counter_Slot_2_C|GetIngredientOnCounterSlot2 _output_get_2) "None")
            (Variables|Default|SetIsBunsPresent false)
            (Variables|Default|SetIsGrilledPattyPresent false)))))
    (:then_2
      (if (Utilities|Enum|Equal(Enum) (Variables|Default|GetCurrentOrder) "Burger")
        (if (Variables|Default|GetIsBunsPresent)
          (if (Variables|Default|GetIsGrilledPattyPresent)
            (Utilities|FlowControl|Sequence
              (:then_0
                (Utilities|IsValid (Variables|/Game/FinalProjectBlueprints/BP_Counter_slot_1.BP_Counter_Slot_1_C|GetBP_Ingredient_Buns_On_Counter_Slot_1 (Variables|Default|GetBP_Counter_Slot_1))
                  (:Is%20Valid
                    (Actor|DestroyActor (Variables|/Game/FinalProjectBlueprints/BP_Counter_slot_1.BP_Counter_Slot_1_C|GetBP_Ingredient_Buns_On_Counter_Slot_1 (Variables|Default|GetBP_Counter_Slot_1))))
                  (:Is%20Not%20Valid
                    (Utilities|IsValid (Variables|/Game/FinalProjectBlueprints/BP_Counter_slot_1.BP_Counter_Slot_1_C|GetBP_Ingredient_Grilled_Patty_On_Counter_Slot_1 (Variables|Default|GetBP_Counter_Slot_1))
                      (:Is%20Valid
                        (Actor|DestroyActor (Variables|/Game/FinalProjectBlueprints/BP_Counter_slot_1.BP_Counter_Slot_1_C|GetBP_Ingredient_Grilled_Patty_On_Counter_Slot_1 (Variables|Default|GetBP_Counter_Slot_1)))))))
                (Variables|/Game/FinalProjectBlueprints/BP_Counter_slot_1.BP_Counter_Slot_1_C|SetIngredientOnCounterSlot1 (Variables|Default|GetBP_Counter_Slot_1) "None"))
              (:then_1
                (Utilities|IsValid (Variables|/Game/FinalProjectBlueprints/BP_Counter_Slot_2.BP_Counter_Slot_2_C|GetBP_Ingredient_Buns_On_Counter_Slot_2 (Variables|Default|GetBP_Counter_Slot_2))
                  (:Is%20Valid
                    (Actor|DestroyActor (Variables|/Game/FinalProjectBlueprints/BP_Counter_Slot_2.BP_Counter_Slot_2_C|GetBP_Ingredient_Buns_On_Counter_Slot_2 (Variables|Default|GetBP_Counter_Slot_2))))
                  (:Is%20Not%20Valid
                    (Utilities|IsValid (Variables|/Game/FinalProjectBlueprints/BP_Counter_Slot_2.BP_Counter_Slot_2_C|GetBP_Ingredient_Grilled_Patty_On_Counter_Slot_2 (Variables|Default|GetBP_Counter_Slot_2))
                      (:Is%20Valid
                        (Actor|DestroyActor (Variables|/Game/FinalProjectBlueprints/BP_Counter_Slot_2.BP_Counter_Slot_2_C|GetBP_Ingredient_Grilled_Patty_On_Counter_Slot_2 (Variables|Default|GetBP_Counter_Slot_2)))))))
                (Variables|/Game/FinalProjectBlueprints/BP_Counter_Slot_2.BP_Counter_Slot_2_C|SetIngredientOnCounterSlot2 (Variables|Default|GetBP_Counter_Slot_2) "None"))
              (:then_2
                (bind _returnvalue_2 (Game|SpawnActorfromClass "/Game/FinalProjectBlueprints/BP_Burger.BP_Burger_C" (Math|Transform|MakeTransform (Math|Vector|MakeVector (.x _returnvalue) (.y _returnvalue) (+ (.z _returnvalue) 1e+02)) "0, 0, 0" "1,1,1") "Undefined" 0 0))
                (Variables|Default|SetBP_Burger_On_Counter_Slot_Finished_Product _returnvalue_2)))))))))

(fn ConstructionScript)