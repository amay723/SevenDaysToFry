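; BP_Counter_Slot_2 is a kitchen counter slot where the player places or picks up a grilled patty or buns.
; Interact compares string states on BP_Character and the slot to choose between placing and picking up.
; Transfers destroy and respawn the ingredient actor, attaching it to the player with collision off on pickup.
; While InteractArrow is visible, Tick plays a self-restarting timeline that offsets the arrow's height.
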(event EventBeginPlay)

(event Collision|EventActorBeginOverlap
  (params (OtherActor :type Actor%20Object%20Reference)))

(event EventTick
  (params (DeltaSeconds :type Float%20%28single-precision%29))
  (bind _interactarrow (Variables|Default|GetInteractArrow))
  (if (Rendering|IsVisible _interactarrow)
    (bind _newtrack_1 (Timeline|Timeline_0 Play)
      (:Update
        (Transformation|SetRelativeLocation _interactarrow (Math|Vector|MakeVector 0.0 0.0 (+ (.x _newtrack_1) (.z (Variables|/Script/Engine.SceneComponent|GetRelativeLocation _interactarrow)))) false false))
      (:Finished
        (if true
          (Timeline|Timeline_0 PlayFromStart))))))

(event EventInteract
  (bind _returnvalue (Transformation|GetActorTransform))
  (bind _returnvalue_2 (Transformation|GetActorLocation))
  (bind _returnvalue_3 (Transformation|GetActorTransform))
  (bind _returnvalue_4 (Transformation|GetActorLocation))
  (bind _asbp_character (Utilities|Casting|CastToBP_Character (Game|GetPlayerCharacter 0)))
  (Variables|Default|SetBP_Character _asbp_character)
  (if (Utilities|Enum|Equal(Enum) (Variables|/Game/FinalProjectBlueprints/BP_Character.BP_Character_C|GetIngredientHeldByPlayer (Variables|Default|GetBP_Character)) "GrilledPatty")
    (bind _returnvalue_5 (Game|SpawnActorfromClass "/Game/RecipeData/Ingredients/BP_Ingredient_Grilled_Patty.BP_Ingredient_Grilled_Patty_C" (Math|Transform|MakeTransform (Math|Vector|MakeVector (.x _returnvalue_2) (.y _returnvalue_2) (+ (.z _returnvalue_2) 103.0)) "0, 0, 0" "1,1,1") "Undefined" 0 0))
    (Variables|Default|SetBP_Ingredient_Grilled_Patty_On_Counter_Slot_2 _returnvalue_5)
    (Utilities|IsValid (Variables|/Game/FinalProjectBlueprints/BP_Character.BP_Character_C|GetBP_Ingredient_Grilled_Patty_Instance (Variables|Default|GetBP_Character))
      (:Is%20Valid
        (Actor|DestroyActor (Variables|/Game/FinalProjectBlueprints/BP_Character.BP_Character_C|GetBP_Ingredient_Grilled_Patty_Instance (Variables|Default|GetBP_Character)))
        (Variables|/Game/FinalProjectBlueprints/BP_Character.BP_Character_C|SetIngredientHeldByPlayer (Variables|Default|GetBP_Character) "None")
        (Variables|Default|SetIngredientOnCounterSlot2 "GrilledPatty")))
    (elif (Utilities|Enum|Equal(Enum) (Variables|/Game/FinalProjectBlueprints/BP_Character.BP_Character_C|GetIngredientHeldByPlayer (Variables|Default|GetBP_Character)) "Buns")
      (bind _returnvalue_6 (Game|SpawnActorfromClass "/Game/RecipeData/Ingredients/BP_Ingredient_Buns.BP_Ingredient_Buns_C" (Math|Transform|MakeTransform (Math|Vector|MakeVector (.x _returnvalue_4) (.y _returnvalue_4) (+ (.z _returnvalue_4) 113.0)) "0, 0, 0" "1,1,1") "Undefined" 0 0))
      (Variables|Default|SetBP_Ingredient_Buns_On_Counter_Slot_2 _returnvalue_6)
      (Utilities|IsValid (Variables|/Game/FinalProjectBlueprints/BP_Character.BP_Character_C|GetBP_Ingredient_Buns_Instance (Variables|Default|GetBP_Character))
        (:Is%20Valid
          (Actor|DestroyActor (Variables|/Game/FinalProjectBlueprints/BP_Character.BP_Character_C|GetBP_Ingredient_Buns_Instance (Variables|Default|GetBP_Character)))
          (Variables|/Game/FinalProjectBlueprints/BP_Character.BP_Character_C|SetIngredientHeldByPlayer (Variables|Default|GetBP_Character) "None")
          (Variables|Default|SetIngredientOnCounterSlot2 "Buns")))
      (elif (Utilities|Enum|Equal(Enum) (Variables|/Game/FinalProjectBlueprints/BP_Character.BP_Character_C|GetIngredientHeldByPlayer (Variables|Default|GetBP_Character)) "None")
        (if (Utilities|Enum|Equal(Enum) (Variables|Default|GetIngredientOnCounterSlot2) "GrilledPatty")
          (Utilities|IsValid (Variables|Default|GetBP_Ingredient_Grilled_Patty_On_Counter_Slot_2)
            (:Is%20Valid
              (Actor|DestroyActor (Variables|Default|GetBP_Ingredient_Grilled_Patty_On_Counter_Slot_2))
              (bind _returnvalue_7 (Game|SpawnActorfromClass "/Game/RecipeData/Ingredients/BP_Ingredient_Grilled_Patty.BP_Ingredient_Grilled_Patty_C" (Math|Transform|MakeTransform (Math|Vector|MakeVector (.x (.location _returnvalue_3)) (.y (.location _returnvalue_3)) (+ (.z (.location _returnvalue_3)) 1e+02)) (.rotation _returnvalue_3) (.scale _returnvalue_3)) "Undefined" 0 0))
              (bind _output_get (Variables|/Game/FinalProjectBlueprints/BP_Character.BP_Character_C|SetBP_Ingredient_Grilled_Patty_Instance (Variables|Default|GetBP_Character) _returnvalue_7))
              (Transformation|AttachActorToActor _returnvalue_7 (Game|GetPlayerCharacter 0) "None" "KeepWorld" "KeepWorld" "KeepWorld" true)
              (Collision|SetActorEnableCollision _output_get false)
              (Variables|/Game/FinalProjectBlueprints/BP_Character.BP_Character_C|SetIngredientHeldByPlayer (Variables|Default|GetBP_Character) "GrilledPatty")
              (Variables|Default|SetIngredientOnCounterSlot2 "None" :!label _label)))
          (elif (Utilities|Enum|Equal(Enum) (Variables|Default|GetIngredientOnCounterSlot2) "Buns")
            (Utilities|IsValid (Variables|Default|GetBP_Ingredient_Buns_On_Counter_Slot_2)
              (:Is%20Valid
                (Actor|DestroyActor (Variables|Default|GetBP_Ingredient_Buns_On_Counter_Slot_2))
                (bind _returnvalue_8 (Game|SpawnActorfromClass "/Game/RecipeData/Ingredients/BP_Ingredient_Buns.BP_Ingredient_Buns_C" (Math|Transform|MakeTransform (Math|Vector|MakeVector (.x (.location _returnvalue)) (.y (.location _returnvalue)) (+ (.z (.location _returnvalue)) 1e+02)) (.rotation _returnvalue) (.scale _returnvalue)) "Undefined" 0 0))
                (bind _output_get_2 (Variables|/Game/FinalProjectBlueprints/BP_Character.BP_Character_C|SetBP_Ingredient_Buns_Instance (Variables|Default|GetBP_Character) _returnvalue_8))
                (Transformation|AttachActorToActor _returnvalue_8 (Game|GetPlayerCharacter 0) "None" "KeepWorld" "KeepWorld" "KeepWorld" true)
                (Collision|SetActorEnableCollision _output_get_2 false)
                (Variables|/Game/FinalProjectBlueprints/BP_Character.BP_Character_C|SetIngredientHeldByPlayer (Variables|Default|GetBP_Character) "Buns")
                (goto _label)))))))))

(fn ConstructionScript)