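; First-person player character for a burger-cooking game with a gun, handling movement, station interaction, shooting, barricade repair and automatic doors.
; Each tick a camera line trace finds interactable actors, shows their arrows and caches them for the Interact handlers.
; A held-item string gates pickups, grilling and firing.
; Any non-negative damage is lethal as written, disabling input and triggering a camera-roll timeline that resets the alive flag when finished.
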(event Custom|GazeCheck
  (bind _camera (Variables|Default|GetCamera))
  (bind _returnvalue (Transformation|GetWorldLocation _camera))
  ;[1 1 1] Gaze check
  (bind _outhit (Collision|LineTraceByChannel _returnvalue (+ _returnvalue (* (Math|Vector|GetForwardVector _camera) 2000)) "TraceTypeQuery1" false 0 "ForOneFrame"))
  (if (Utilities|DoesObjectImplementInterface (.HitActor (Collision|BreakHitResult _outhit)) "/Game/FinalProjectBlueprints/BP_Interactive_Interface.BP_Interactive_Interface_C")
    (bind _asgun (Utilities|Casting|CastTogun (.HitActor (Collision|BreakHitResult _outhit)))
      (:then
        (bind _output_get (Variables|Default|Setgun _asgun))
        (Rendering|SetVisibility (Variables|/Game/gun.gun_C|GetInteractArrow _output_get) true false))
      (:CastFailed
        (bind _asbp_grill (Utilities|Casting|CastToBP_Grill (.HitActor (Collision|BreakHitResult _outhit)))
          (:then
            (bind _output_get_2 (Variables|Default|SetBP_Grill _asbp_grill))
            (Rendering|SetVisibility (Variables|/Game/FinalProjectBlueprints/BP_Grill.BP_Grill_C|GetInteractArrow _output_get_2) true false))
          (:CastFailed
            (bind _asbp_ingredient_patty_spawner (Utilities|Casting|CastToBP_Ingredient_Patty_Spawner (.HitActor (Collision|BreakHitResult _outhit)))
              (:then
                (bind _output_get_3 (Variables|Default|SetBP_Ingredient_Patty_Spawner _asbp_ingredient_patty_spawner))
                (Rendering|SetVisibility (Variables|/Game/RecipeData/Ingredients/BP_Ingredient_Patty_Spawner.BP_Ingredient_Patty_Spawner_C|GetInteractArrow _output_get_3) true false)
                (Utilities|IsValid (Variables|Default|GetBP_Ingredient_Buns_Spawner)
                  (:Is%20Valid
                    (Rendering|SetVisibility (Variables|/Game/RecipeData/Ingredients/BP_Ingredient_Buns_Spawner.BP_Ingredient_Buns_Spawner_C|GetInteractArrow (Variables|Default|GetBP_Ingredient_Buns_Spawner)) false false)
                    (Variables|Default|SetBP_Ingredient_Buns_Spawner 0))))
              (:CastFailed
                (Utilities|IsValid (Variables|Default|GetBP_Ingredient_Patty_Spawner)
                  (:Is%20Valid
                    (Rendering|SetVisibility (Variables|/Game/RecipeData/Ingredients/BP_Ingredient_Patty_Spawner.BP_Ingredient_Patty_Spawner_C|GetInteractArrow (Variables|Default|GetBP_Ingredient_Patty_Spawner)) false false)
                    (Variables|Default|SetBP_Ingredient_Patty_Spawner 0))
                  (:Is%20Not%20Valid
                    _))
                (bind _asbp_ingredient_buns_spawner (Utilities|Casting|CastToBP_Ingredient_Buns_Spawner (.HitActor (Collision|BreakHitResult _outhit)))
                  (:then
                    (bind _output_get_4 (Variables|Default|SetBP_Ingredient_Buns_Spawner _asbp_ingredient_buns_spawner))
                    (Rendering|SetVisibility (Variables|/Game/RecipeData/Ingredients/BP_Ingredient_Buns_Spawner.BP_Ingredient_Buns_Spawner_C|GetInteractArrow _output_get_4) true false))
                  (:CastFailed
                    (bind _asbp_counter_slot_1 (Utilities|Casting|CastToBP_Counter_Slot_1 (.HitActor (Collision|BreakHitResult _outhit)))
                      (:then
                        (bind _output_get_5 (Variables|Default|SetBP_Counter_Slot_1 _asbp_counter_slot_1))
                        (Variables|Default|SetBP_Counter_Slot_1_Instance _output_get_5)
                        (Rendering|SetVisibility (Variables|/Game/FinalProjectBlueprints/BP_Counter_slot_1.BP_Counter_Slot_1_C|GetInteractArrow _output_get_5) true false)
                        (Utilities|IsValid (Variables|Default|GetBP_Counter_Slot_2)
                          (:Is%20Valid
                            (Rendering|SetVisibility (Variables|/Game/FinalProjectBlueprints/BP_Counter_Slot_2.BP_Counter_Slot_2_C|GetInteractArrow (Variables|Default|GetBP_Counter_Slot_2)) false false)
                            (Variables|Default|SetBP_Counter_Slot_2 0))))
                      (:CastFailed
                        (Utilities|IsValid (Variables|Default|GetBP_Counter_Slot_1)
                          (:Is%20Valid
                            (Rendering|SetVisibility (Variables|/Game/FinalProjectBlueprints/BP_Counter_slot_1.BP_Counter_Slot_1_C|GetInteractArrow (Variables|Default|GetBP_Counter_Slot_1)) false false)
                            (Variables|Default|SetBP_Counter_Slot_1 0))
                          (:Is%20Not%20Valid
                            _))
                        (bind _asbp_counter_slot_2 (Utilities|Casting|CastToBP_Counter_Slot_2 (.HitActor (Collision|BreakHitResult _outhit)))
                          (:then
                            (bind _output_get_6 (Variables|Default|SetBP_Counter_Slot_2 _asbp_counter_slot_2))
                            (Variables|Default|SetBP_Counter_Slot_2_Instance _output_get_6)
                            (Rendering|SetVisibility (Variables|/Game/FinalProjectBlueprints/BP_Counter_Slot_2.BP_Counter_Slot_2_C|GetInteractArrow _output_get_6) true false))
                          (:CastFailed
                            (Utilities|IsValid (Variables|Default|GetBP_Counter_Slot_2)
                              (:Is%20Valid
                                (Rendering|SetVisibility (Variables|/Game/FinalProjectBlueprints/BP_Counter_Slot_2.BP_Counter_Slot_2_C|GetInteractArrow (Variables|Default|GetBP_Counter_Slot_2)) false false)
                                (Variables|Default|SetBP_Counter_Slot_2 0))
                              (:Is%20Not%20Valid
                                _))
                            (bind _asbp_trashcan (Utilities|Casting|CastToBP_Trashcan (.HitActor (Collision|BreakHitResult _outhit))))
                            (bind _output_get_7 (Variables|Default|SetBP_Trashcan _asbp_trashcan))
                            (Rendering|SetVisibility (Variables|/Game/FinalProjectBlueprints/BP_Trashcan.BP_Trashcan_C|GetInteractArrow _output_get_7) true false)))))))))))))
    (else
      (Utilities|FlowControl|Sequence
        (:then_0
          (Utilities|IsValid (Variables|Default|GetBP_Grill)
            (:Is%20Valid
              (Rendering|SetVisibility (Variables|/Game/FinalProjectBlueprints/BP_Grill.BP_Grill_C|GetInteractArrow (Variables|Default|GetBP_Grill)) false false)
              (Variables|Default|SetBP_Grill 0))))
        (:then_1
          (Utilities|IsValid (Variables|Default|GetBP_Counter_Slot_1)
            (:Is%20Valid
              (Rendering|SetVisibility (Variables|/Game/FinalProjectBlueprints/BP_Counter_slot_1.BP_Counter_Slot_1_C|GetInteractArrow (Variables|Default|GetBP_Counter_Slot_1)) false false)
              (Variables|Default|SetBP_Counter_Slot_1 0))))
        (:then_2
          (Utilities|IsValid (Variables|Default|GetBP_Counter_Slot_2)
            (:Is%20Valid
              (Rendering|SetVisibility (Variables|/Game/FinalProjectBlueprints/BP_Counter_Slot_2.BP_Counter_Slot_2_C|GetInteractArrow (Variables|Default|GetBP_Counter_Slot_2)) false false)
              (Variables|Default|SetBP_Counter_Slot_2 0))))
        (:then_3
          (Utilities|IsValid (Variables|Default|GetBP_Ingredient_Buns_Spawner)
            (:Is%20Valid
              (Rendering|SetVisibility (Variables|/Game/RecipeData/Ingredients/BP_Ingredient_Buns_Spawner.BP_Ingredient_Buns_Spawner_C|GetInteractArrow (Variables|Default|GetBP_Ingredient_Buns_Spawner)) false false)
              (Variables|Default|SetBP_Ingredient_Buns_Spawner 0))))
        (:then_4
          (Utilities|IsValid (Variables|Default|GetBP_Ingredient_Patty_Spawner)
            (:Is%20Valid
              (Rendering|SetVisibility (Variables|/Game/RecipeData/Ingredients/BP_Ingredient_Patty_Spawner.BP_Ingredient_Patty_Spawner_C|GetInteractArrow (Variables|Default|GetBP_Ingredient_Patty_Spawner)) false false)
              (Variables|Default|SetBP_Ingredient_Patty_Spawner 0))))
        (:then_5
          (Utilities|IsValid (Variables|Default|GetBP_Trashcan)
            (:Is%20Valid
              (Rendering|SetVisibility (Variables|/Game/FinalProjectBlueprints/BP_Trashcan.BP_Trashcan_C|GetInteractArrow (Variables|Default|GetBP_Trashcan)) false false)
              (Variables|Default|SetBP_Trashcan 0))))
        (:then_6
          (Utilities|IsValid (Variables|Default|Getgun)
            (:Is%20Valid
              (Rendering|SetVisibility (Variables|/Game/gun.gun_C|GetInteractArrow (Variables|Default|Getgun)) false false)
              (Variables|Default|Setgun 0))))))))

(event Custom|CustomEvent
  ;[1 1 1] Begin Play
  (bind _outactors (Actor|GetAllActorsOfClass "/Game/FinalProjectBlueprints/BP_Counter_Slot_Finished_Product.BP_Counter_Slot_Finished_Product_C"))
  (Variables|Default|SetBP_Counter_Slot_Finished_Product (Utilities|Array|Get(acopy) _outactors))
  (bind _outactors_2 (Actor|GetAllActorsOfClass "/Game/FinalProjectBlueprints/BP_Counter_slot_1.BP_Counter_Slot_1_C"))
  (Variables|Default|SetBP_Counter_Slot_1_Instance (Utilities|Array|Get(acopy) _outactors_2))
  (bind _outactors_3 (Actor|GetAllActorsOfClass "/Game/FinalProjectBlueprints/BP_Counter_Slot_2.BP_Counter_Slot_2_C"))
  (Variables|Default|SetBP_Counter_Slot_2_Instance (Utilities|Array|Get(acopy) _outactors_3)))

(event EventTick
  (params (DeltaSeconds :type Float%20%28single-precision%29))
  ;[1 1 1] Tick
  (CallFunction|GazeCheck)
  (if (not (Variables|Default|GetisAlive))
    (bind _newtrack_1 (Timeline|Deathrattle Play)
      (:Update
        (Transformation|SetRelativeRotation (Variables|Default|GetCamera) (Math|Rotator|MakeRotator (.x _newtrack_1) 0.0 0.0) false false))
      (:Finished
        (Variables|Default|SetisAlive true)))))

(event Collision|EventActorBeginOverlap
  (params (OtherActor :type Actor%20Object%20Reference))
  ;[1 1 1] AutomaticDoor
  (bind _asbp_user_door (Utilities|Casting|CastToBP_UserDoor OtherActor))
  (Default|ActivateDoor _asbp_user_door))

(event Game|Damage|EventAnyDamage
  (params (Damage :type Float%20%28single-precision%29) (DamageType :type Damage%20Type%20Object%20Reference) (InstigatedBy :type Controller%20Object%20Reference) (DamageCauser :type Actor%20Object%20Reference))
  (|CallParentFunction Damage DamageType InstigatedBy DamageCauser)
  ;[1 1 1] Apply Damage
  (if (>= Damage 0.0)
    (bind _output_get (Variables|Default|SetCharacterHealth (- 0.0 Damage)))
    ;[1 1 1] Character is Dead
    (if (<= _output_get 0.0)
      (Input|DisableInput 0)
      (Variables|Default|SetisAlive false)
      (Development|PrintString "You Died!"))))

(event Input|ActionEvents|InputActionshoot
  (params (Key :type Key%20Structure))
  ;[1 1 1] Shoot da gun
  (:Pressed
    (if (and (Variables|Default|GetCanFire) (Utilities|Enum|Equal(Enum) (Variables|Default|GetIngredientHeldByPlayer) "Gun"))
      (bind _outactors (Actor|GetAllActorsOfClass "/Game/gun.gun_C"))
      (Default|Fire (Utilities|Array|Get(acopy) _outactors)))))

(event Input|ActionEvents|InputActionInteract
  (params (Key :type Key%20Structure))
  (bind _bp_counter_slot_2 (Variables|Default|GetBP_Counter_Slot_2))
  (bind _bp_counter_slot_finished_product (Variables|Default|GetBP_Counter_Slot_Finished_Product))
  ;[1 1 1] Counter Slot Interactions
  (:Pressed
    (Utilities|IsValid _bp_counter_slot_2
      (:Is%20Valid
        (Class|BPInteractiveInterface|Interact(Message) _bp_counter_slot_2)
        (Utilities|IsValid _bp_counter_slot_finished_product
          (:Is%20Valid
            (Class|BPInteractiveInterface|Interact(Message) _bp_counter_slot_finished_product)))))))

(event Input|ActionEvents|InputActionInteract
  (params (Key :type Key%20Structure))
  (bind _bp_ingredient_patty_spawner (Variables|Default|GetBP_Ingredient_Patty_Spawner))
  ;[1 1 1] Pick Up Raw Ingredients
  (:Pressed
    (Utilities|IsValid _bp_ingredient_patty_spawner
      (:Is%20Valid
        (if (Utilities|Enum|Equal(Enum) (Variables|Default|GetIngredientHeldByPlayer) "None")
          (Class|BPInteractiveInterface|Interact(Message) _bp_ingredient_patty_spawner)
          (Variables|Default|SetIngredientHeldByPlayer "Patty")
          (Variables|Default|SetBP_Ingredient_Patty_Instance (Variables|/Game/RecipeData/Ingredients/BP_Ingredient_Patty_Spawner.BP_Ingredient_Patty_Spawner_C|GetBP_Ingredient_Patty_Instance (Variables|Default|GetBP_Ingredient_Patty_Spawner))))))))

(event Input|ActionEvents|InputActionInteract
  (params (Key :type Key%20Structure))
  (bind _bp_counter_slot_1 (Variables|Default|GetBP_Counter_Slot_1))
  (bind _bp_counter_slot_finished_product (Variables|Default|GetBP_Counter_Slot_Finished_Product))
  ;[1 1 1] Counter Slot Interactions
  (:Pressed
    (Utilities|IsValid _bp_counter_slot_1
      (:Is%20Valid
        (Class|BPInteractiveInterface|Interact(Message) _bp_counter_slot_1)
        (Utilities|IsValid _bp_counter_slot_finished_product
          (:Is%20Valid
            (Class|BPInteractiveInterface|Interact(Message) _bp_counter_slot_finished_product)))))))

(event Input|ActionEvents|InputActionInteract
  (params (Key :type Key%20Structure))
  ;[1 1 1] Grill Interactions
  (:Pressed
    (Utilities|IsValid (Variables|Default|GetBP_Grill)
      (:Is%20Valid
        (if (Utilities|Enum|Equal(Enum) (Variables|Default|GetIngredientHeldByPlayer) "Patty")
          (Actor|DestroyActor (Variables|Default|GetBP_Ingredient_Patty_Instance))
          (Class|BPInteractiveInterface|Interact(Message) (Variables|Default|GetBP_Grill))
          (Variables|Default|SetIngredientHeldByPlayer "None")
          (Variables|Default|SetBP_Grill 0)
          (elif (Utilities|Enum|Equal(Enum) (Variables|Default|GetIngredientHeldByPlayer) "None")
            (Class|BPInteractiveInterface|Interact(Message) (Variables|Default|GetBP_Grill))
            (if (Variables|/Game/FinalProjectBlueprints/BP_Grill.BP_Grill_C|GetIsPattyCooked (Variables|Default|GetBP_Grill))
              (Variables|Default|SetBP_Ingredient_Grilled_Patty_Instance (Variables|/Game/FinalProjectBlueprints/BP_Grill.BP_Grill_C|GetBP_Ingredient_Grilled_Patty_Instance (Variables|Default|GetBP_Grill)))
              (Variables|Default|SetIngredientHeldByPlayer "GrilledPatty")
              (Variables|/Game/FinalProjectBlueprints/BP_Grill.BP_Grill_C|SetIsPattyCooked (Variables|Default|GetBP_Grill) false))))))))

(event Input|ActionEvents|InputActionInteract
  (params (Key :type Key%20Structure))
  (bind _bp_trashcan (Variables|Default|GetBP_Trashcan))
  ;[1 1 1] Trashcan
  (:Pressed
    (Utilities|IsValid _bp_trashcan
      (:Is%20Valid
        (Class|BPInteractiveInterface|Interact(Message) _bp_trashcan)))))

(event Input|ActionEvents|InputActionFixBarricade
  (params (Key :type Key%20Structure))
  ;[1 1 1] Buyables
  ;;[1 1 1] Barricade Fix
  (:Pressed
    (bind _asbp_game_mode (Utilities|Casting|CastToBP_GameMode (Game|GetGameMode)))
    (Default|RecreateBarricade _asbp_game_mode)))

(event Input|ActionEvents|InputActionInteract
  (params (Key :type Key%20Structure))
  (bind _bp_ingredient_buns_spawner (Variables|Default|GetBP_Ingredient_Buns_Spawner))
  ;[1 1 1] Pick Up Raw Ingredients
  (:Pressed
    (Utilities|IsValid _bp_ingredient_buns_spawner
      (:Is%20Valid
        (if (Utilities|Enum|Equal(Enum) (Variables|Default|GetIngredientHeldByPlayer) "None")
          (Class|BPInteractiveInterface|Interact(Message) _bp_ingredient_buns_spawner)
          (Variables|Default|SetIngredientHeldByPlayer "Buns")
          (Variables|Default|SetBP_Ingredient_Buns_Instance (Variables|/Game/RecipeData/Ingredients/BP_Ingredient_Buns_Spawner.BP_Ingredient_Buns_Spawner_C|GetBP_Ingredient_Buns_Instance (Variables|Default|GetBP_Ingredient_Buns_Spawner))))))))

(event Input|ActionEvents|InputActionInteract
  (params (Key :type Key%20Structure))
  (bind _gun (Variables|Default|Getgun))
  (bind _gun_2 (Variables|Default|Getgun))
  ;[1 1 1] Pickup Gun
  (:Pressed
    (Utilities|IsValid _gun_2
      (:Is%20Valid
        (Development|PrintString "gun test")
        (if (Utilities|Enum|Equal(Enum) (Variables|Default|GetIngredientHeldByPlayer) "None")
          (Class|BPInteractiveInterface|Interact(Message) _gun_2)
          (Development|PrintString "gun test 2")
          (Variables|Default|SetIngredientHeldByPlayer "Gun")
          (bind _output_get (Variables|Default|Setgun_instance (Variables|/Game/gun.gun_C|Getgun_instance _gun)))
          (Transformation|SetActorLocation _output_get (+ (Transformation|GetActorLocation _gun) "70.000000, 0,-50.000000") false false))))))

(event Input|AxisEvents|InputAxismouseX
  (params (AxisValue :type Float%20%28single-precision%29))
  ;[1 1 1] FinalProject Inputs
  (Pawn|Input|AddControllerYawInput AxisValue))

(event Input|AxisEvents|InputAxismouseY
  (params (AxisValue :type Float%20%28single-precision%29))
  ;[1 1 1] FinalProject Inputs
  (Pawn|Input|AddControllerPitchInput AxisValue))

(event Input|AxisEvents|InputAxisMoveForward
  (params (AxisValue :type Float%20%28single-precision%29))
  ;[1 1 1] FinalProject Inputs
  (Pawn|Input|AddMovementInput (Transformation|GetActorForwardVector) AxisValue false))

(event Input|AxisEvents|InputAxisMoveRight
  (params (AxisValue :type Float%20%28single-precision%29))
  ;[1 1 1] FinalProject Inputs
  (Pawn|Input|AddMovementInput (Transformation|GetActorRightVector) AxisValue false))

(fn ConstructionScript)

(fn Die
  (if (Variables|Default|GetisAlive)
    (Variables|Default|SetisAlive false)
    (if (not (Variables|Default|GetSound_Played))
      (Audio|PlaySoundatLocation 0 "0, 0, 0" "0, 0, 0" 5.0 1.0 0.2 0 0 0)
      (Variables|Default|SetSound_Played true))))