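; First-person player character for a burger-cooking game, handling movement, look and item interaction.
; Tick runs a camera line trace that caches the interactable patty, grill, counter or buns under the gaze.
; Interact handlers use those references and held-item flags to carry ingredients, grill patties and combine them with buns on the counter.
; Die plays a sound once and flags death, prompting Tick to roll the camera via the Deathrattle timeline.
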(event Custom|GazeCheck
  (bind _camera (Variables|Default|GetCamera))
  (bind _returnvalue (Transformation|GetWorldLocation _camera))
  ;[1 1 1] Gaze check
  (bind _outhit (Collision|LineTraceByChannel _returnvalue (+ _returnvalue (* (Math|Vector|GetForwardVector _camera) 2000)) "TraceTypeQuery1" false 0 "ForOneFrame"))
  (if (Utilities|DoesObjectImplementInterface (.HitActor (Collision|BreakHitResult _outhit)) "/Game/FinalProjectBlueprints/BP_Interactive_Interface.BP_Interactive_Interface_C")
    (bind _asbp_patty (Utilities|Casting|CastToBP_Patty (.HitActor (Collision|BreakHitResult _outhit)))
      (:then
        (Variables|Default|SetBP_Patty _asbp_patty))
      (:CastFailed
        (bind _asbp_grill (Utilities|Casting|CastToBP_Grill (.HitActor (Collision|BreakHitResult _outhit)))
          (:then
            (Variables|Default|SetBP_Grill _asbp_grill))
          (:CastFailed
            (bind _asbp_counter (Utilities|Casting|CastToBP_Counter (.HitActor (Collision|BreakHitResult _outhit)))
              (:then
                (Variables|Default|SetBP_Counter _asbp_counter))
              (:CastFailed
                (bind _asbp_buns (Utilities|Casting|CastToBP_Buns (.HitActor (Collision|BreakHitResult _outhit))))
                (Variables|Default|SetBP_Buns _asbp_buns)))))))
    (else
      (Utilities|FlowControl|Sequence
        (:then_0
          (Variables|Default|SetBP_Patty 0))
        (:then_1
          (Variables|Default|SetBP_Grill 0))
        (:then_2
          (Variables|Default|SetBP_Counter 0))
        (:then_3
          (Variables|Default|SetBP_Buns 0))))))

(event EventBeginPlay)

(event EventTick
  (params (DeltaSeconds :type Float%20%28single-precision%29))
  ;[1 1 1] Tick
  (CallFunction|GazeCheck)
  (if (Variables|Default|GetI_AM_DEAD)
    (bind _newtrack_1 (Timeline|Deathrattle Play)
      (:Update
        (Transformation|SetRelativeRotation (Variables|Default|GetCamera) (Math|Rotator|MakeRotator (.x _newtrack_1) 0.0 0.0) false false))
      (:Finished
        (Variables|Default|SetI_AM_DEAD false)))))

(event Input|ActionEvents|InputActionInteract
  (params (Key :type Key%20Structure))
  (bind _bp_counter (Variables|Default|GetBP_Counter))
  (bind _bp_counter_2 (Variables|Default|GetBP_Counter))
  (bind _bp_buns_instance (Variables|Default|GetBP_Buns_Instance))
  (bind _bp_grilled_patty_on_counter (Variables|/Game/FinalProjectBlueprints/BP_Counter.BP_Counter_C|GetBP_Grilled_Patty_On_Counter _bp_counter_2))
  ;[1 1 1] Counter Interactions
  (:Pressed
    (Utilities|IsValid _bp_counter
      (:Is%20Valid
        (if (Variables|Default|GetIsBunsBeingHeld)
          (if (Variables|Default|GetIsGrilledPattyOnCounter)
            (Variables|Default|SetIsBurgerCompleted true))
          (Class|BPInteractiveInterface|Interact(Message) _bp_counter)
          (Utilities|IsValid _bp_buns_instance
            (:Is%20Valid
              (Actor|DestroyActor _bp_buns_instance)
              (Variables|Default|SetIsBunsBeingHeld false)
              (if (Variables|Default|GetIsBurgerCompleted)
                (Utilities|IsValid _bp_grilled_patty_on_counter
                  (:Is%20Valid
                    (Actor|DestroyActor _bp_grilled_patty_on_counter)))
                (else
                  (Variables|Default|SetIsBunsOnCounter true))))))))))

(event Input|ActionEvents|InputActionInteract
  (params (Key :type Key%20Structure))
  ;[1 1 1] Grill Interactions
  (:Pressed
    (Utilities|IsValid (Variables|Default|GetBP_Grill)
      (:Is%20Valid
        (if (Variables|Default|GetIsPattyBeingHeld)
          (Actor|DestroyActor (Variables|Default|GetBP_Patty_Instance))
          (Class|BPInteractiveInterface|Interact(Message) (Variables|Default|GetBP_Grill))
          (Variables|Default|SetIsPattyBeingHeld false)
          (Variables|Default|SetBP_Grill 0)
          (else
            (Class|BPInteractiveInterface|Interact(Message) (Variables|Default|GetBP_Grill))
            (Variables|Default|SetBP_Grilled_Patty_Instance (Variables|/Game/FinalProjectBlueprints/BP_Grill.BP_Grill_C|GetBP_Grilled_Patty_Instance (Variables|Default|GetBP_Grill)))
            (Variables|Default|SetIsGrilledPattyBeingHeld true)))))))

(event Input|ActionEvents|InputActionInteract
  (params (Key :type Key%20Structure))
  ;[1 1 1] Pick Up Raw Ingredients
  (:Pressed
    (Utilities|IsValid (Variables|Default|GetBP_Patty)
      (:Is%20Valid
        (if (not (Variables|Default|GetIsPattyBeingHeld))
          (Class|BPInteractiveInterface|Interact(Message) (Variables|Default|GetBP_Patty))
          (Variables|Default|SetIsPattyBeingHeld true)
          (Variables|Default|SetBP_Patty_Instance (Variables|/Game/FinalProjectBlueprints/BP_Patty.BP_Patty_C|GetBP_Patty_Instance (Variables|Default|GetBP_Patty)))
          (Variables|Default|SetBP_Patty 0)
          (Variables|Default|SetIsHandEmpty false))))))

(event Input|ActionEvents|InputActionInteract
  (params (Key :type Key%20Structure))
  ;[1 1 1] Pick Up Raw Ingredients
  (:Pressed
    (Utilities|IsValid (Variables|Default|GetBP_Buns)
      (:Is%20Valid
        (if (not (Variables|Default|GetIsBunsBeingHeld))
          (Class|BPInteractiveInterface|Interact(Message) (Variables|Default|GetBP_Buns))
          (Variables|Default|SetIsBunsBeingHeld true)
          (Variables|Default|SetBP_Buns_Instance (Variables|/Game/FinalProjectBlueprints/BP_Buns.BP_Buns_C|GetBP_Buns_Instance (Variables|Default|GetBP_Buns)))
          (Variables|Default|SetBP_Buns 0)
          (Variables|Default|SetIsHandEmpty false))))))

(event Input|ActionEvents|InputActionInteract
  (params (Key :type Key%20Structure))
  ;[1 1 1] Counter Interactions
  (:Pressed
    (Utilities|IsValid (Variables|Default|GetBP_Counter))))

(event Input|ActionEvents|InputActionInteract
  (params (Key :type Key%20Structure))
  (bind _bp_counter (Variables|Default|GetBP_Counter))
  (bind _bp_grilled_patty_instance (Variables|Default|GetBP_Grilled_Patty_Instance))
  (bind _bp_counter_2 (Variables|Default|GetBP_Counter))
  (bind _bp_buns_on_counter (Variables|/Game/FinalProjectBlueprints/BP_Counter.BP_Counter_C|GetBP_Buns_On_Counter _bp_counter_2))
  ;[1 1 1] Counter Interactions
  (:Pressed
    (Utilities|IsValid _bp_counter
      (:Is%20Valid
        (if (Variables|Default|GetIsGrilledPattyBeingHeld)
          (if (Variables|Default|GetIsBunsOnCounter)
            (Variables|Default|SetIsBurgerCompleted true))
          (Class|BPInteractiveInterface|Interact(Message) _bp_counter)
          (Utilities|IsValid _bp_grilled_patty_instance
            (:Is%20Valid
              (Actor|DestroyActor _bp_grilled_patty_instance)
              (Variables|Default|SetIsGrilledPattyBeingHeld false)
              (if (Variables|Default|GetIsBurgerCompleted)
                (Utilities|IsValid _bp_buns_on_counter
                  (:Is%20Valid
                    (Actor|DestroyActor _bp_buns_on_counter)))
                (else
                  (Variables|Default|SetIsGrilledPattyOnCounter true))))))))))

(event Input|AxisEvents|InputAxismouseX
  (params (AxisValue :type Float%20%28single-precision%29))
  ;[1 1 1] FinalProject Inputs
  (Pawn|Input|AddControllerYawInput AxisValue))

(event Input|AxisEvents|InputAxismouseY
  (params (AxisValue :type Float%20%28single-precision%29))
  ;[1 1 1] FinalProject Inputs
  (Pawn|Input|AddControllerPitchInput AxisValue))

(event Input|AxisEvents|InputAxisMoveForward
  (params (AxisValue :type Float%20%28single-precision%29))
  ;[1 1 1] FinalProject Inputs
  (Pawn|Input|AddMovementInput (Transformation|GetActorForwardVector) AxisValue false))

(event Input|AxisEvents|InputAxisMoveRight
  (params (AxisValue :type Float%20%28single-precision%29))
  ;[1 1 1] FinalProject Inputs
  (Pawn|Input|AddMovementInput (Transformation|GetActorRightVector) AxisValue false))

(fn ConstructionScript)

(fn Die
  (if (not (Variables|Default|GetI_AM_DEAD))
    (Variables|Default|SetI_AM_DEAD true)
    (if (not (Variables|Default|GetSound_Played))
      (Audio|PlaySoundatLocation 0 "0, 0, 0" "0, 0, 0" 5.0 1.0 0.2 0 0 0)
      (Variables|Default|SetSound_Played true))))