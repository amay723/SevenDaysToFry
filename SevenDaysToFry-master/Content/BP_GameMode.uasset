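; BP_GameMode is a game mode Blueprint that sets up the main HUD and counts waves.
; BeginPlay creates the Main_HUD widget, stores it and adds it to the viewport.
; Each Tick reads GameTime, incrementing WaveCount when it reaches an upper threshold.
; The WaveCheck flag latches that increment until GameTime falls to a lower threshold; nothing in these graphs updates GameTime itself.
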(event EventBeginPlay
  (bind _returnvalue (UserInterface|CreateWidget "/Game/HUD/Main_HUD.Main_HUD_C"))
  (bind _output_get (Variables|Default|SetMain_HUD _returnvalue))
  (UserInterface|Viewport|AddtoViewport _output_get 0))

(event EventTick
  (params (DeltaSeconds :type Float%20%28single-precision%29))
  (Utilities|FlowControl|Sequence
    (:then_0
      ;[1 1 1] Wave Set and Checks
      (if (Variables|Default|GetWaveCheck)
        (if (<= (Variables|Default|GetGameTime) 1e+02)
          (Variables|Default|SetWaveCheck false))
        (elif (>= (Variables|Default|GetGameTime) 8e+02)
          (Variables|Default|SetWaveCount (+ (Variables|Default|GetWaveCount) 1))
          (Variables|Default|SetWaveCheck true))))))

(fn ConstructionScript)