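; BP_Trashcan is an interactable trashcan that discards the ingredient the player is carrying.
; Interact reads the held ingredient from BP_Character, destroys the first valid buns, grilled patty or patty instance, and resets the held name to "None".
; While the interact arrow is visible, Tick plays a self-restarting timeline that animates it vertically by adding the track value to its current relative Z.
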(event EventBeginPlay)

(event Collision|EventActorBeginOverlap
  (params (OtherActor :type Actor%20Object%20Reference)))

(event EventTick
  (params (DeltaSeconds :type Float%20%28single-precision%29))
  (bind _interactarrow (Variables|Default|GetInteractArrow))
  (if (Rendering|IsVisible _interactarrow)
    (bind _newtrack_1 (Timeline|Timeline_0 Play)
      (:Update
        (Transformation|SetRelativeLocation _interactarrow (Math|Vector|MakeVector 0.0 0.0 (+ (.x _newtrack_1) (.z (Variables|/Script/Engine.SceneComponent|GetRelativeLocation _interactarrow)))) false false))
      (:Finished
        (if true
          (Timeline|Timeline_0 PlayFromStart))))))

(event EventInteract
  (bind _asbp_character (Utilities|Casting|CastToBP_Character (Game|GetPlayerCharacter 0)))
  (Variables|Default|SetBP_Character _asbp_character)
  (if (Utilities|Enum|NotEqual(Enum) (Variables|/Game/FinalProjectBlueprints/BP_Character.BP_Character_C|GetIngredientHeldByPlayer _asbp_character) "None")
    (Utilities|IsValid (Variables|/Game/FinalProjectBlueprints/BP_Character.BP_Character_C|GetBP_Ingredient_Buns_Instance (Variables|Default|GetBP_Character))
      (:Is%20Valid
        (Actor|DestroyActor (Variables|/Game/FinalProjectBlueprints/BP_Character.BP_Character_C|GetBP_Ingredient_Buns_Instance (Variables|Default|GetBP_Character))))
      (:Is%20Not%20Valid
        (Utilities|IsValid (Variables|/Game/FinalProjectBlueprints/BP_Character.BP_Character_C|GetBP_Ingredient_Grilled_Patty_Instance (Variables|Default|GetBP_Character))
          (:Is%20Valid
            (Actor|DestroyActor (Variables|/Game/FinalProjectBlueprints/BP_Character.BP_Character_C|GetBP_Ingredient_Grilled_Patty_Instance (Variables|Default|GetBP_Character))))
          (:Is%20Not%20Valid
            (Utilities|IsValid (Variables|/Game/FinalProjectBlueprints/BP_Character.BP_Character_C|GetBP_Ingredient_Patty_Instance (Variables|Default|GetBP_Character))
              (:Is%20Valid
                (Actor|DestroyActor (Variables|/Game/FinalProjectBlueprints/BP_Character.BP_Character_C|GetBP_Ingredient_Patty_Instance (Variables|Default|GetBP_Character)))))))))
    (Variables|/Game/FinalProjectBlueprints/BP_Character.BP_Character_C|SetIngredientHeldByPlayer (Variables|Default|GetBP_Character) "None")))

(fn ConstructionScript)