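; BP_Counter_Slot_Finished_Product is an interactable counter slot that assembles a burger from buns and a grilled patty.
; On Interact, it reads ingredient flags and the two counter slot instances from BP_Character, accepting the pair in either arrangement.
; It destroys both ingredient actors after validity checks, then spawns a BP_Burger above itself and stores the reference.
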(event EventBeginPlay)

(event Collision|EventActorBeginOverlap
  (params (OtherActor :type Actor%20Object%20Reference)))

(event EventTick
  (params (DeltaSeconds :type Float%20%28single-precision%29)))

(event EventInteract
  (bind _returnvalue (Transformation|GetActorLocation))
  (bind _asbp_character (Utilities|Casting|CastToBP_Character (Game|GetPlayerCharacter 0)))
  (Variables|Default|SetIsBunsOnCounterSlot1 (Variables|/Game/FinalProjectBlueprints/BP_Character.BP_Character_C|GetIsBunsOnCounterSlot1 _asbp_character))
  (Variables|Default|SetIsBunsOnCounterSlot2 (Variables|/Game/FinalProjectBlueprints/BP_Character.BP_Character_C|GetIsBunsOnCounterSlot2 _asbp_character))
  (Variables|Default|SetIsGrilledPattyOnCounterSlot1 (Variables|/Game/FinalProjectBlueprints/BP_Character.BP_Character_C|GetIsGrilledPattyOnCounterSlot1 _asbp_character))
  (Variables|Default|SetIsGrilledPattyOnCounterSlot2 (Variables|/Game/FinalProjectBlueprints/BP_Character.BP_Character_C|GetIsGrilledPattyOnCounterSlot2 _asbp_character))
  (Variables|Default|SetBP_Counter_Slot_1 (Variables|/Game/FinalProjectBlueprints/BP_Character.BP_Character_C|GetBP_Counter_Slot_1_Instance _asbp_character))
  (Variables|Default|SetBP_Counter_Slot_2 (Variables|/Game/FinalProjectBlueprints/BP_Character.BP_Character_C|GetBP_Counter_Slot_2_Instance _asbp_character))
  (if (Variables|Default|GetIsBunsOnCounterSlot1)
    (if (Variables|Default|GetIsGrilledPattyOnCounterSlot2)
      (Utilities|IsValid (Variables|/Game/FinalProjectBlueprints/BP_Counter_slot_1.BP_Counter_Slot_1_C|GetBP_Buns_On_Counter_Slot_1 (Variables|Default|GetBP_Counter_Slot_1))
        (:Is%20Valid
          (Actor|DestroyActor (Variables|/Game/FinalProjectBlueprints/BP_Counter_slot_1.BP_Counter_Slot_1_C|GetBP_Buns_On_Counter_Slot_1 (Variables|Default|GetBP_Counter_Slot_1)))
          (Utilities|IsValid (Variables|/Game/FinalProjectBlueprints/BP_Counter_Slot_2.BP_Counter_Slot_2_C|GetBP_Grilled_Patty_On_Counter_Slot_2 (Variables|Default|GetBP_Counter_Slot_2))
            (:Is%20Valid
              (Actor|DestroyActor (Variables|/Game/FinalProjectBlueprints/BP_Counter_Slot_2.BP_Counter_Slot_2_C|GetBP_Grilled_Patty_On_Counter_Slot_2 (Variables|Default|GetBP_Counter_Slot_2)))
              (bind _returnvalue_2 (Game|SpawnActorfromClass "/Game/FinalProjectBlueprints/BP_Burger.BP_Burger_C" (Math|Transform|MakeTransform (Math|Vector|MakeVector (.x _returnvalue) (.y _returnvalue) (+ (.z _returnvalue) 1e+02)) "0, 0, 0" "1,1,1") "Undefined" 0 0 :!label _label))
              (Variables|Default|SetBP_Burger_On_Counter_Slot_Finished_Product _returnvalue_2))))))
    (elif (Variables|Default|GetIsGrilledPattyOnCounterSlot1)
      (if (Variables|Default|GetIsBunsOnCounterSlot2)
        (Utilities|IsValid (Variables|/Game/FinalProjectBlueprints/BP_Counter_slot_1.BP_Counter_Slot_1_C|GetBP_Grilled_Patty_On_Counter_Slot_1 (Variables|Default|GetBP_Counter_Slot_1))
          (:Is%20Valid
            (Actor|DestroyActor (Variables|/Game/FinalProjectBlueprints/BP_Counter_slot_1.BP_Counter_Slot_1_C|GetBP_Grilled_Patty_On_Counter_Slot_1 (Variables|Default|GetBP_Counter_Slot_1)))
            (Utilities|IsValid (Variables|/Game/FinalProjectBlueprints/BP_Counter_Slot_2.BP_Counter_Slot_2_C|GetBP_Buns_On_Counter_Slot_2 (Variables|Default|GetBP_Counter_Slot_2))
              (:Is%20Valid
                (Actor|DestroyActor (Variables|/Game/FinalProjectBlueprints/BP_Counter_Slot_2.BP_Counter_Slot_2_C|GetBP_Buns_On_Counter_Slot_2 (Variables|Default|GetBP_Counter_Slot_2)))
                (goto _label)))))))))

(fn ConstructionScript)