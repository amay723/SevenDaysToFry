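; BP_Counter is a kitchen counter that places a copy of the food the player is holding on top of itself.
; On Interact, it checks BP_Character's flags in priority order: completed burger, grilled patty, then buns.
; The first match spawns that item at a per-item height above the counter and stores a reference to it.
; It neither changes the character's held-item flags nor checks whether the counter is already occupied.
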(event EventBeginPlay)

(event Collision|EventActorBeginOverlap
  (params (OtherActor :type Actor%20Object%20Reference)))

(event EventTick
  (params (DeltaSeconds :type Float%20%28single-precision%29)))

(event EventInteract
  (bind _returnvalue (Transformation|GetActorLocation))
  (bind _returnvalue_2 (Transformation|GetActorLocation))
  (bind _returnvalue_3 (Transformation|GetActorLocation))
  (bind _asbp_character (Utilities|Casting|CastToBP_Character (Game|GetPlayerCharacter 0)))
  (if (Variables|/Game/FinalProjectBlueprints/BP_Character.BP_Character_C|GetIsBurgerCompleted _asbp_character)
    (bind _returnvalue_4 (Game|SpawnActorfromClass "/Game/FinalProjectBlueprints/BP_Burger.BP_Burger_C" (Math|Transform|MakeTransform (Math|Vector|MakeVector (.x _returnvalue_2) (.y _returnvalue_2) (+ (.z _returnvalue_2) 1e+02)) "0, 0, 0" "1,1,1") "Undefined" 0 0))
    (Variables|Default|SetBP_Burger_On_Counter _returnvalue_4)
    (elif (Variables|/Game/FinalProjectBlueprints/BP_Character.BP_Character_C|GetIsGrilledPattyBeingHeld _asbp_character)
      (bind _returnvalue_5 (Game|SpawnActorfromClass "/Game/FinalProjectBlueprints/BP_Grilled_Patty.BP_Grilled_Patty_C" (Math|Transform|MakeTransform (Math|Vector|MakeVector (.x _returnvalue) (.y _returnvalue) (+ (.z _returnvalue) 103.0)) "0, 0, 0" "1,1,1") "Undefined" 0 0))
      (Variables|Default|SetBP_Grilled_Patty_On_Counter _returnvalue_5)
      (elif (Variables|/Game/FinalProjectBlueprints/BP_Character.BP_Character_C|GetIsBunsBeingHeld _asbp_character)
        (bind _returnvalue_6 (Game|SpawnActorfromClass "/Game/FinalProjectBlueprints/BP_Buns.BP_Buns_C" (Math|Transform|MakeTransform (Math|Vector|MakeVector (.x _returnvalue_3) (.y _returnvalue_3) (+ (.z _returnvalue_3) 113.0)) "0, 0, 0" "1.000000,1.000000,1.000000") "Undefined" 0 0))
        (Variables|Default|SetBP_Buns_On_Counter _returnvalue_6)))))

(fn ConstructionScript)