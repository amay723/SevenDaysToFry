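; BP_UserDoor is a door that swings open when its ActivateDoor event is called and closes itself shortly after.
; The DoorOpenClose timeline drives the Door component's relative yaw, playing forward to open and in reverse to close.
; IsFinished ignores activations during a swing, and IsOpen picks the direction.
; When a swing finishes, a short delay re-triggers ActivateDoor if the door is still open.
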(event Custom|ActivateDoor
  (if (Variables|Default|GetbIsFinished)
    (Variables|Default|SetbIsFinished false)
    (if (Variables|Default|GetbIsOpen)
      (Variables|Default|SetbIsOpen false)
      (bind _rotation (Timeline|DoorOpenClose ReverseFromEnd)
        (:Update
          (Transformation|SetRelativeRotation (Variables|Default|GetDoor) (Math|Rotator|MakeRotator 0.0 0.0 (.z _rotation)) false false))
        (:Finished
          (Variables|Default|SetbIsFinished true)
          (Utilities|FlowControl|Delay 0.5)
          (if (Variables|Default|GetbIsOpen)
            (CallFunction|ActivateDoor))))
      (else
        (Variables|Default|SetbIsOpen true)
        (Timeline|DoorOpenClose PlayFromStart)))))

(event EventBeginPlay)

(event Collision|EventActorBeginOverlap
  (params (OtherActor :type Actor%20Object%20Reference)))

(event EventTick
  (params (DeltaSeconds :type Float%20%28single-precision%29)))

(fn ConstructionScript)