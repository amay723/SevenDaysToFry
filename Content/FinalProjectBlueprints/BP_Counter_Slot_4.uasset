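; Counter slot 4 in a burger kitchen, where the player drops off or picks up one ingredient through Interact.
; A held ingredient is respawned above the slot and the held instance destroyed; empty hands destroy the slot's item and attach a fresh, collision-free copy to the character.
; Each ingredient type has its own branch, and the empty-slot check is unwired, so placing ignores occupancy.
; Tick drives a looping timeline that moves InteractArrow vertically while visible.
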(event EventBeginPlay)

(event Collision|EventActorBeginOverlap
  (params (OtherActor :type Actor%20Object%20Reference)))

(event EventTick
  (params (DeltaSeconds :type Float%20%28single-precision%29))
  (bind _interactarrow (Variables|Default|GetInteractArrow))
  (if (Rendering|IsVisible _interactarrow)
    (bind _newtrack_1 (Timeline|Timeline_0 Play)
      (:Update
        (Transformation|SetRelativeLocation _interactarrow (Math|Vector|MakeVector 0.0 0.0 (+ (.x _newtrack_1) (.z (Variables|/Script/Engine.SceneComponent|GetRelativeLocation _interactarrow)))) false false))
      (:Finished
        (if true
          (Timeline|Timeline_0 PlayFromStart))))))

(event EventInteract
  (bind _returnvalue (Transformation|GetActorTransform))
  (bind _returnvalue_2 (Transformation|GetActorLocation))
  (bind _returnvalue_3 (Transformation|GetActorLocation))
  (bind _returnvalue_4 (Transformation|GetActorTransform))
  (bind _returnvalue_5 (Transformation|GetActorTransform))
  (bind _returnvalue_6 (Transformation|GetActorLocation))
  (bind _returnvalue_7 (Transformation|GetActorTransform))
  (bind _returnvalue_8 (Transformation|GetActorLocation))
  (bind _returnvalue_9 (Transformation|GetActorTransform))
  (bind _returnvalue_10 (Transformation|GetActorLocation))
  (bind _returnvalue_11 (Transformation|GetActorLocation))
  (bind _returnvalue_12 (Transformation|GetActorLocation))
  (bind _returnvalue_13 (Transformation|GetActorTransform))
  (bind _returnvalue_14 (Transformation|GetActorTransform))
  (bind _asbp_character (Utilities|Casting|CastToBP_Character (Game|GetPlayerCharacter 0)))
  (Variables|Default|SetBP_Character _asbp_character)
  (switch string (Variables|/Game/FinalProjectBlueprints/BP_Character.BP_Character_C|GetIngredientHeldByPlayer (Variables|Default|GetBP_Character))
    (:GrilledPatty
      (bind _returnvalue_15 (Game|SpawnActorfromClass "/Game/RecipeData/Ingredients/BP_Ingredient_Grilled_Patty.BP_Ingredient_Grilled_Patty_C" (Math|Transform|MakeTransform (Math|Vector|MakeVector (.x _returnvalue_2) (.y _returnvalue_2) (+ (.z _returnvalue_2) 87.0)) "0, 0, 0" "1,1,1") "Undefined" 0 0))
      (Variables|Default|SetBP_Ingredient_Grilled_Patty_On_Counter_Slot_4 _returnvalue_15)
      (Utilities|IsValid (Variables|/Game/FinalProjectBlueprints/BP_Character.BP_Character_C|GetBP_Ingredient_Grilled_Patty_Instance (Variables|Default|GetBP_Character))
        (:Is%20Valid
          (Actor|DestroyActor (Variables|/Game/FinalProjectBlueprints/BP_Character.BP_Character_C|GetBP_Ingredient_Grilled_Patty_Instance (Variables|Default|GetBP_Character)))
          (Variables|/Game/FinalProjectBlueprints/BP_Character.BP_Character_C|SetIngredientHeldByPlayer (Variables|Default|GetBP_Character) "None")
          (Variables|Default|SetIngredientOnCounterSlot4 "GrilledPatty"))))
    (:Buns
      (bind _returnvalue_16 (Game|SpawnActorfromClass "/Game/RecipeData/Ingredients/BP_Ingredient_Buns.BP_Ingredient_Buns_C" (Math|Transform|MakeTransform (Math|Vector|MakeVector (.x _returnvalue_3) (.y _returnvalue_3) (+ (.z _returnvalue_3) 9e+01)) "0, 0, 0" "1,1,1") "Undefined" 0 0))
      (Variables|Default|SetBP_Ingredient_Buns_On_Counter_Slot_4 _returnvalue_16)
      (Utilities|IsValid (Variables|/Game/FinalProjectBlueprints/BP_Character.BP_Character_C|GetBP_Ingredient_Buns_Instance (Variables|Default|GetBP_Character))
        (:Is%20Valid
          (Actor|DestroyActor (Variables|/Game/FinalProjectBlueprints/BP_Character.BP_Character_C|GetBP_Ingredient_Buns_Instance (Variables|Default|GetBP_Character)))
          (Variables|/Game/FinalProjectBlueprints/BP_Character.BP_Character_C|SetIngredientHeldByPlayer (Variables|Default|GetBP_Character) "None")
          (Variables|Default|SetIngredientOnCounterSlot4 "Buns"))))
    (:Cheese
      (bind _returnvalue_17 (Game|SpawnActorfromClass "/Game/RecipeData/Ingredients/BP_Ingredient_Cheese.BP_Ingredient_Cheese_C" (Math|Transform|MakeTransform (Math|Vector|MakeVector (.x _returnvalue_6) (.y _returnvalue_6) (+ (.z _returnvalue_6) 87.0)) "0, 0, 0" "1,1,1") "Undefined" 0 0))
      (Variables|Default|SetBP_Ingredient_Cheese_On_Counter_Slot_4 _returnvalue_17)
      (Utilities|IsValid (Variables|/Game/FinalProjectBlueprints/BP_Character.BP_Character_C|GetBP_Ingredient_Cheese_Instance (Variables|Default|GetBP_Character))
        (:Is%20Valid
          (Actor|DestroyActor (Variables|/Game/FinalProjectBlueprints/BP_Character.BP_Character_C|GetBP_Ingredient_Cheese_Instance (Variables|Default|GetBP_Character)))
          (Variables|/Game/FinalProjectBlueprints/BP_Character.BP_Character_C|SetIngredientHeldByPlayer (Variables|Default|GetBP_Character) "None")
          (Variables|Default|SetIngredientOnCounterSlot4 "Cheese"))))
    (:Lettuce
      (bind _returnvalue_18 (Game|SpawnActorfromClass "/Game/RecipeData/Ingredients/BP_Ingredient_Lettuce.BP_Ingredient_Lettuce_C" (Math|Transform|MakeTransform (Math|Vector|MakeVector (.x _returnvalue_8) (.y _returnvalue_8) (+ (.z _returnvalue_8) 87.0)) "0, 0, 0" "1,1,1") "Undefined" 0 0))
      (Variables|Default|SetBP_Ingredient_Lettuce_On_Counter_Slot_4 _returnvalue_18)
      (Utilities|IsValid (Variables|/Game/FinalProjectBlueprints/BP_Character.BP_Character_C|GetBP_Ingredient_Lettuce_Instance (Variables|Default|GetBP_Character))
        (:Is%20Valid
          (Actor|DestroyActor (Variables|/Game/FinalProjectBlueprints/BP_Character.BP_Character_C|GetBP_Ingredient_Lettuce_Instance (Variables|Default|GetBP_Character)))
          (Variables|/Game/FinalProjectBlueprints/BP_Character.BP_Character_C|SetIngredientHeldByPlayer (Variables|Default|GetBP_Character) "None")
          (Variables|Default|SetIngredientOnCounterSlot4 "Lettuce"))))
    (:Pickles
      (bind _returnvalue_19 (Game|SpawnActorfromClass "/Game/RecipeData/Ingredients/BP_Ingredient_Pickles.BP_Ingredient_Pickles_C" (Math|Transform|MakeTransform (Math|Vector|MakeVector (.x _returnvalue_10) (.y _returnvalue_10) (+ (.z _returnvalue_10) 87.0)) "0, 0, 0" "1,1,1") "Undefined" 0 0))
      (Variables|Default|SetBP_Ingredient_Pickles_On_Counter_Slot_4 _returnvalue_19)
      (Utilities|IsValid (Variables|/Game/FinalProjectBlueprints/BP_Character.BP_Character_C|GetBP_Ingredient_Pickles_Instance (Variables|Default|GetBP_Character))
        (:Is%20Valid
          (Actor|DestroyActor (Variables|/Game/FinalProjectBlueprints/BP_Character.BP_Character_C|GetBP_Ingredient_Pickles_Instance (Variables|Default|GetBP_Character)))
          (Variables|/Game/FinalProjectBlueprints/BP_Character.BP_Character_C|SetIngredientHeldByPlayer (Variables|Default|GetBP_Character) "None")
          (Variables|Default|SetIngredientOnCounterSlot4 "Pickles"))))
    (:Onions
      (bind _returnvalue_20 (Game|SpawnActorfromClass "/Game/RecipeData/Ingredients/BP_Ingredient_Onions.BP_Ingredient_Onions_C" (Math|Transform|MakeTransform (Math|Vector|MakeVector (.x _returnvalue_11) (.y _returnvalue_11) (+ (.z _returnvalue_11) 87.0)) "0, 0, 0" "1,1,1") "Undefined" 0 0))
      (Variables|Default|SetBP_Ingredient_Onions_On_Counter_Slot_4 _returnvalue_20)
      (Utilities|IsValid (Variables|/Game/FinalProjectBlueprints/BP_Character.BP_Character_C|GetBP_Ingredient_Onions_Instance (Variables|Default|GetBP_Character))
        (:Is%20Valid
          (Actor|DestroyActor (Variables|/Game/FinalProjectBlueprints/BP_Character.BP_Character_C|GetBP_Ingredient_Onions_Instance (Variables|Default|GetBP_Character)))
          (Variables|/Game/FinalProjectBlueprints/BP_Character.BP_Character_C|SetIngredientHeldByPlayer (Variables|Default|GetBP_Character) "None")
          (Variables|Default|SetIngredientOnCounterSlot4 "Onions"))))
    (:GrilledBacon
      (bind _returnvalue_21 (Game|SpawnActorfromClass "/Game/RecipeData/Ingredients/BP_Ingredient_Grilled_Bacon.BP_Ingredient_Grilled_Bacon_C" (Math|Transform|MakeTransform (Math|Vector|MakeVector (.x _returnvalue_12) (.y _returnvalue_12) (+ (.z _returnvalue_12) 87.0)) "0, 0, 0" "1,1,1") "Undefined" 0 0))
      (Variables|Default|SetBP_Ingredient_Grilled_Bacon_On_Counter_Slot_4 _returnvalue_21)
      (Utilities|IsValid (Variables|/Game/FinalProjectBlueprints/BP_Character.BP_Character_C|GetBP_Ingredient_Grilled_Bacon_Instance (Variables|Default|GetBP_Character))
        (:Is%20Valid
          (Actor|DestroyActor (Variables|/Game/FinalProjectBlueprints/BP_Character.BP_Character_C|GetBP_Ingredient_Grilled_Bacon_Instance (Variables|Default|GetBP_Character)))
          (Variables|/Game/FinalProjectBlueprints/BP_Character.BP_Character_C|SetIngredientHeldByPlayer (Variables|Default|GetBP_Character) "None")
          (Variables|Default|SetIngredientOnCounterSlot4 "GrilledBacon"))))
    (:None
      (switch string (Variables|Default|GetIngredientOnCounterSlot4)
        (:GrilledPatty
          (Utilities|IsValid (Variables|Default|GetBP_Ingredient_Grilled_Patty_On_Counter_Slot_4)
            (:Is%20Valid
              (Actor|DestroyActor (Variables|Default|GetBP_Ingredient_Grilled_Patty_On_Counter_Slot_4))
              (bind _returnvalue_22 (Game|SpawnActorfromClass "/Game/RecipeData/Ingredients/BP_Ingredient_Grilled_Patty.BP_Ingredient_Grilled_Patty_C" (Math|Transform|MakeTransform (Math|Vector|MakeVector (.x (.location _returnvalue_5)) (.y (.location _returnvalue_5)) (+ (.z (.location _returnvalue_5)) 87.0)) (.rotation _returnvalue_5) (.scale _returnvalue_5)) "Undefined" 0 0))
              (bind _output_get (Variables|/Game/FinalProjectBlueprints/BP_Character.BP_Character_C|SetBP_Ingredient_Grilled_Patty_Instance (Variables|Default|GetBP_Character) _returnvalue_22))
              (Transformation|AttachActorToActor _returnvalue_22 (Game|GetPlayerCharacter 0) "None" "KeepWorld" "KeepWorld" "KeepWorld" true)
              (Collision|SetActorEnableCollision _output_get false)
              (Variables|/Game/FinalProjectBlueprints/BP_Character.BP_Character_C|SetIngredientHeldByPlayer (Variables|Default|GetBP_Character) "GrilledPatty"))))
        (:Buns
          (Utilities|IsValid (Variables|Default|GetBP_Ingredient_Buns_On_Counter_Slot_4)
            (:Is%20Valid
              (Actor|DestroyActor (Variables|Default|GetBP_Ingredient_Buns_On_Counter_Slot_4))
              (bind _returnvalue_23 (Game|SpawnActorfromClass "/Game/RecipeData/Ingredients/BP_Ingredient_Buns.BP_Ingredient_Buns_C" (Math|Transform|MakeTransform (Math|Vector|MakeVector (.x (.location _returnvalue_4)) (.y (.location _returnvalue_4)) (+ (.z (.location _returnvalue_4)) 9e+01)) (.rotation _returnvalue_4) (.scale _returnvalue_4)) "Undefined" 0 0))
              (bind _output_get_2 (Variables|/Game/FinalProjectBlueprints/BP_Character.BP_Character_C|SetBP_Ingredient_Buns_Instance (Variables|Default|GetBP_Character) _returnvalue_23))
              (Transformation|AttachActorToActor _returnvalue_23 (Game|GetPlayerCharacter 0) "None" "KeepWorld" "KeepWorld" "KeepWorld" true)
              (Collision|SetActorEnableCollision _output_get_2 false)
              (Variables|/Game/FinalProjectBlueprints/BP_Character.BP_Character_C|SetIngredientHeldByPlayer (Variables|Default|GetBP_Character) "Buns"))))
        (:Cheese
          (Utilities|IsValid (Variables|Default|GetBP_Ingredient_Cheese_On_Counter_Slot_4)
            (:Is%20Valid
              (Actor|DestroyActor (Variables|Default|GetBP_Ingredient_Cheese_On_Counter_Slot_4))
              (bind _returnvalue_24 (Game|SpawnActorfromClass "/Game/RecipeData/Ingredients/BP_Ingredient_Cheese.BP_Ingredient_Cheese_C" (Math|Transform|MakeTransform (Math|Vector|MakeVector (.x (.location _returnvalue_7)) (.y (.location _returnvalue_7)) (+ (.z (.location _returnvalue_7)) 87.0)) (.rotation _returnvalue_7) (.scale _returnvalue_7)) "Undefined" 0 0))
              (bind _output_get_3 (Variables|/Game/FinalProjectBlueprints/BP_Character.BP_Character_C|SetBP_Ingredient_Cheese_Instance (Variables|Default|GetBP_Character) _returnvalue_24))
              (Transformation|AttachActorToActor _returnvalue_24 (Game|GetPlayerCharacter 0) "None" "KeepWorld" "KeepWorld" "KeepWorld" true)
              (Collision|SetActorEnableCollision _output_get_3 false)
              (Variables|/Game/FinalProjectBlueprints/BP_Character.BP_Character_C|SetIngredientHeldByPlayer (Variables|Default|GetBP_Character) "Cheese"))))
        (:Lettuce
          (Utilities|IsValid (Variables|Default|GetBP_Ingredient_Lettuce_On_Counter_Slot_4)
            (:Is%20Valid
              (Actor|DestroyActor (Variables|Default|GetBP_Ingredient_Lettuce_On_Counter_Slot_4))
              (bind _returnvalue_25 (Game|SpawnActorfromClass "/Game/RecipeData/Ingredients/BP_Ingredient_Lettuce.BP_Ingredient_Lettuce_C" (Math|Transform|MakeTransform (Math|Vector|MakeVector (.x (.location _returnvalue_9)) (.y (.location _returnvalue_9)) (+ (.z (.location _returnvalue_9)) 87.0)) (.rotation _returnvalue_9) (.scale _returnvalue_9)) "Undefined" 0 0))
              (bind _output_get_4 (Variables|/Game/FinalProjectBlueprints/BP_Character.BP_Character_C|SetBP_Ingredient_Lettuce_Instance (Variables|Default|GetBP_Character) _returnvalue_25))
              (Transformation|AttachActorToActor _returnvalue_25 (Game|GetPlayerCharacter 0) "None" "KeepWorld" "KeepWorld" "KeepWorld" true)
              (Collision|SetActorEnableCollision _output_get_4 false)
              (Variables|/Game/FinalProjectBlueprints/BP_Character.BP_Character_C|SetIngredientHeldByPlayer (Variables|Default|GetBP_Character) "Lettuce"))))
        (:Pickles
          (Utilities|IsValid (Variables|Default|GetBP_Ingredient_Pickles_On_Counter_Slot_4)
            (:Is%20Valid
              (Actor|DestroyActor (Variables|Default|GetBP_Ingredient_Pickles_On_Counter_Slot_4))
              (bind _returnvalue_26 (Game|SpawnActorfromClass "/Game/RecipeData/Ingredients/BP_Ingredient_Pickles.BP_Ingredient_Pickles_C" (Math|Transform|MakeTransform (Math|Vector|MakeVector (.x (.location _returnvalue_13)) (.y (.location _returnvalue_13)) (+ (.z (.location _returnvalue_13)) 87.0)) (.rotation _returnvalue_13) (.scale _returnvalue_13)) "Undefined" 0 0))
              (bind _output_get_5 (Variables|/Game/FinalProjectBlueprints/BP_Character.BP_Character_C|SetBP_Ingredient_Pickles_Instance (Variables|Default|GetBP_Character) _returnvalue_26))
              (Transformation|AttachActorToActor _returnvalue_26 (Game|GetPlayerCharacter 0) "None" "KeepWorld" "KeepWorld" "KeepWorld" true)
              (Collision|SetActorEnableCollision _output_get_5 false)
              (Variables|/Game/FinalProjectBlueprints/BP_Character.BP_Character_C|SetIngredientHeldByPlayer (Variables|Default|GetBP_Character) "Pickles"))))
        (:Onions
          (Utilities|IsValid (Variables|Default|GetBP_Ingredient_Onions_On_Counter_Slot_4)
            (:Is%20Valid
              (Actor|DestroyActor (Variables|Default|GetBP_Ingredient_Onions_On_Counter_Slot_4))
              (bind _returnvalue_27 (Game|SpawnActorfromClass "/Game/RecipeData/Ingredients/BP_Ingredient_Onions.BP_Ingredient_Onions_C" (Math|Transform|MakeTransform (Math|Vector|MakeVector (.x (.location _returnvalue_14)) (.y (.location _returnvalue_14)) (+ (.z (.location _returnvalue_14)) 87.0)) (.rotation _returnvalue_14) (.scale _returnvalue_14)) "Undefined" 0 0))
              (bind _output_get_6 (Variables|/Game/FinalProjectBlueprints/BP_Character.BP_Character_C|SetBP_Ingredient_Onions_Instance (Variables|Default|GetBP_Character) _returnvalue_27))
              (Transformation|AttachActorToActor _returnvalue_27 (Game|GetPlayerCharacter 0) "None" "KeepWorld" "KeepWorld" "KeepWorld" true)
              (Collision|SetActorEnableCollision _output_get_6 false)
              (Variables|/Game/FinalProjectBlueprints/BP_Character.BP_Character_C|SetIngredientHeldByPlayer (Variables|Default|GetBP_Character) "Onions"))))
        (:GrilledBacon
          (Utilities|IsValid (Variables|Default|GetBP_Ingredient_Grilled_Bacon_On_Counter_Slot_4)
            (:Is%20Valid
              (Actor|DestroyActor (Variables|Default|GetBP_Ingredient_Grilled_Bacon_On_Counter_Slot_4))
              (bind _returnvalue_28 (Game|SpawnActorfromClass "/Game/RecipeData/Ingredients/BP_Ingredient_Grilled_Bacon.BP_Ingredient_Grilled_Bacon_C" (Math|Transform|MakeTransform (Math|Vector|MakeVector (.x (.location _returnvalue)) (.y (.location _returnvalue)) (+ (.z (.location _returnvalue)) 87.0)) (.rotation _returnvalue) (.scale _returnvalue)) "Undefined" 0 0))
              (bind _output_get_7 (Variables|/Game/FinalProjectBlueprints/BP_Character.BP_Character_C|SetBP_Ingredient_Grilled_Bacon_Instance (Variables|Default|GetBP_Character) _returnvalue_28))
              (Transformation|AttachActorToActor _returnvalue_28 (Game|GetPlayerCharacter 0) "None" "KeepWorld" "KeepWorld" "KeepWorld" true)
              (Collision|SetActorEnableCollision _output_get_7 false)
              (Variables|/Game/FinalProjectBlueprints/BP_Character.BP_Character_C|SetIngredientHeldByPlayer (Variables|Default|GetBP_Character) "GrilledBacon")))))
      (Variables|Default|SetIngredientOnCounterSlot4 "None"))))

(fn ConstructionScript)