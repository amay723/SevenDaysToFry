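; BP_Grill is an interactable grill where the player places a held patty and later picks up a grilled one.
; Interact spawns a BP_Grilled_Patty above the grill if the character holds a patty, storing its transform with no cook timer.
; If a patty is already on the grill, Interact destroys it and spawns a replacement at that transform, attached to the player with collision disabled.
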(event EventBeginPlay)

(event Collision|EventActorBeginOverlap
  (params (OtherActor :type Actor%20Object%20Reference)))

(event EventTick
  (params (DeltaSeconds :type Float%20%28single-precision%29)))

(event EventInteract
  (bind _returnvalue (Transformation|GetActorLocation))
  (bind _asbp_character (Utilities|Casting|CastToBP_Character (Game|GetPlayerCharacter 0)))
  (if (Variables|Default|GetIsPattyOnGrill)
    (Actor|DestroyActor (stale _returnvalue_3))
    (Variables|Default|SetIsPattyOnGrill false)
    (bind _returnvalue_2 (Game|SpawnActorfromClass "/Game/FinalProjectBlueprints/BP_Grilled_Patty.BP_Grilled_Patty_C" (Variables|Default|GetPattyOnGrillTransform) "Undefined" 0 0))
    (bind _output_get (Variables|Default|SetBP_Grilled_Patty_Instance _returnvalue_2))
    (Transformation|AttachActorToActor _output_get (Game|GetPlayerCharacter 0) "None" "KeepWorld" "KeepWorld" "KeepWorld" true)
    (Collision|SetActorEnableCollision _output_get false)
    (elif (Variables|/Game/FinalProjectBlueprints/BP_Character.BP_Character_C|GetIsPattyBeingHeld _asbp_character)
      (bind _returnvalue_3 (Game|SpawnActorfromClass "/Game/FinalProjectBlueprints/BP_Grilled_Patty.BP_Grilled_Patty_C" (Math|Transform|MakeTransform (Math|Vector|MakeVector (.x _returnvalue) (.y _returnvalue) (+ (.z _returnvalue) 9e+01)) "0, 0, 0" "1,1,1") "Undefined" 0 0))
      (Variables|Default|SetIsPattyOnGrill true)
      (Variables|Default|SetPattyOnGrillTransform (Transformation|GetActorTransform _returnvalue_3)))))

(fn ConstructionScript)