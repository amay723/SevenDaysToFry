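; BP_Counter is a kitchen counter actor with an indicator arrow that bobs while visible.
; Tick plays the MoveUpAndDown timeline, which offsets the arrow's relative Z and restarts itself when finished.
; The Interact event is empty.
; Disconnected logic reads the player character's held-item flags to spawn a burger, grilled patty or buns above the counter and store the reference, but never runs.
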(event EventBeginPlay)

(event Collision|EventActorBeginOverlap
  (params (OtherActor :type Actor%20Object%20Reference)))

(event EventTick
  (params (DeltaSeconds :type Float%20%28single-precision%29))
  (bind _interactarrow (Variables|Default|GetInteractArrow))
  (if (Rendering|IsVisible _interactarrow)
    (bind _newtrack_1 (Timeline|MoveUpAndDown Play)
      (:Update
        (Transformation|SetRelativeLocation _interactarrow (Math|Vector|MakeVector 0.0 0.0 (+ (.x _newtrack_1) (.z (Variables|/Script/Engine.SceneComponent|GetRelativeLocation _interactarrow)))) false false))
      (:Finished
        (if true
          (Timeline|MoveUpAndDown PlayFromStart))))))

(event EventInteract)

(fn ConstructionScript)