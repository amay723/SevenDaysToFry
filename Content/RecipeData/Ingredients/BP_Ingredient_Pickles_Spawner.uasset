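; Pickles ingredient spawner that hands the player a BP_Ingredient_Pickles when they interact with it.
; Interact calls Equip on BP_Character, stores the returned instance and attaches it to the player.
; Every Tick refreshes a "Pickles" label, shown only when the player is nearby and rotated to face them.
; While InteractArrow is visible, Tick also plays a self-restarting timeline that offsets the arrow's height.
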(event EventBeginPlay)

(event Collision|EventActorBeginOverlap
  (params (OtherActor :type Actor%20Object%20Reference)))

(event EventTick
  (params (DeltaSeconds :type Float%20%28single-precision%29))
  (bind _interactarrow (Variables|Default|GetInteractArrow))
  (CallFunction|Name)
  (if (Rendering|IsVisible _interactarrow)
    (bind _newtrack_1 (Timeline|Timeline_0 Play)
      (:Update
        (Transformation|SetRelativeLocation _interactarrow (Math|Vector|MakeVector 0.0 0.0 (+ (.x _newtrack_1) (.z (Variables|/Script/Engine.SceneComponent|GetRelativeLocation _interactarrow)))) false false))
      (:Finished
        (if true
          (Timeline|Timeline_0 PlayFromStart))))))

(event EventInteract
  (bind _returnvalue (Game|GetPlayerCharacter 0))
  (bind _asbp_character (Utilities|Casting|CastToBP_Character _returnvalue))
  (bind _actor_spawned (Default|Equip _asbp_character (Variables|Default|GetBP_Ingredient_Pickles_Instance) "/Game/RecipeData/Ingredients/BP_Ingredient_Pickles.BP_Ingredient_Pickles_C"))
  (bind _asbp_ingredient_pickles (Utilities|Casting|CastToBP_Ingredient_Pickles _actor_spawned))
  (bind _output_get (Variables|Default|SetBP_Ingredient_Pickles_Instance _asbp_ingredient_pickles))
  (Transformation|AttachActorToActor _output_get _returnvalue "None" "KeepWorld" "KeepWorld" "KeepWorld" true))

(fn ConstructionScript)

(fn Name
  (Rendering|Components|TextRender|SetText (Variables|Default|GetTextRender) (Utilities|Text|FormatText "Pickles"))
  (Rendering|SetVisibility (Variables|Default|GetTextRender) (<= (Math|Vector|VectorLength (- (Transformation|GetActorLocation (Game|GetPlayerCharacter 0)) (Transformation|GetActorLocation))) 3e+02) false)
  (Transformation|SetWorldRotation (Variables|Default|GetTextRender) (Math|Rotator|FindLookatRotation (Transformation|GetActorLocation) (Transformation|GetActorLocation (Game|GetPlayerCharacter 0))) false false))