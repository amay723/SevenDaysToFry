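; Interactable window that opens and closes two curtains with a sound, toggled by Interact or by the GameMode's monster trigger.
; Tick polls the Monstertriggered flag on BP_GameMode and runs the same toggle as Interact, gated by IsFinished to block retriggering mid-animation.
; One timeline plays forward or in reverse to scale and slide both curtains, then re-arms the toggle and clears the monster flag on finish.
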(event EventBeginPlay)

(event Collision|EventActorBeginOverlap
  (params (OtherActor :type Actor%20Object%20Reference)))

(event EventTick
  (params (DeltaSeconds :type Float%20%28single-precision%29))
  (bind _asbp_game_mode (Utilities|Casting|CastToBP_GameMode (Game|GetGameMode)))
  (if (Variables|/Game/Blueprints/BP_GameMode.BP_GameMode_C|Getmonstertriggered _asbp_game_mode)
    (if (Variables|Default|Getis_finished)
      (Variables|Default|Setis_finished false)
      (if (Variables|Default|Getis_open)
        (Variables|Default|Setis_open false)
        (Audio|PlaySoundatLocation "/Game/Sounds/348590__alienxxx__close-curtains.348590__alienxxx__close-curtains" "0, 0, 0" "0, 0, 0" 1.0 1.0 0.0 0 0 0)
        (bind (_direction _newtrack_2 _newtrack_0 _newtrack_1 _newtrack_3) (Timeline|Timeline_1 ReverseFromEnd)
          (:Update
            (Transformation|SetWorldScale3D (Variables|Default|Getcurtain1) (Math|Vector|MakeVector (.x _newtrack_0) 0.04 1.5))
            (Transformation|SetWorldScale3D (Variables|Default|Getcurtain2) (Math|Vector|MakeVector (.x _newtrack_0) 0.04 1.5))
            (Transformation|SetRelativeLocation (Variables|Default|Getcurtain1) (Math|Vector|MakeVector (.x _newtrack_3) 4.0 86.0) false false)
            (Transformation|SetRelativeLocation (Variables|Default|Getcurtain2) (Math|Vector|MakeVector (.x _newtrack_1) 4.0 86.0) false false))
          (:Finished
            (Variables|Default|Setis_finished true)
            (Variables|/Game/Blueprints/BP_GameMode.BP_GameMode_C|Setmonstertriggered _asbp_game_mode false)))
        (else
          (Variables|Default|Setis_open true)
          (Audio|PlaySoundatLocation "/Game/Sounds/348590__alienxxx__close-curtains.348590__alienxxx__close-curtains" "0, 0, 0" "0, 0, 0" 1.0 1.0 0.0 0 0 0)
          (Timeline|Timeline_1 PlayFromStart))))))

(event EventInteract
  (if (Variables|Default|Getis_finished)
    (Variables|Default|Setis_finished false)
    (if (Variables|Default|Getis_open)
      (Variables|Default|Setis_open false)
      (Audio|PlaySoundatLocation "/Game/Sounds/348590__alienxxx__close-curtains.348590__alienxxx__close-curtains" "0, 0, 0" "0, 0, 0" 1.0 1.0 0.0 0 0 0)
      (bind (_direction _newtrack_2 _newtrack_0 _newtrack_1 _newtrack_3) (Timeline|Timeline_1 ReverseFromEnd)
        (:Update
          (Transformation|SetWorldScale3D (Variables|Default|Getcurtain1) (Math|Vector|MakeVector (.x _newtrack_0) 0.04 1.5))
          (Transformation|SetWorldScale3D (Variables|Default|Getcurtain2) (Math|Vector|MakeVector (.x _newtrack_0) 0.04 1.5))
          (Transformation|SetRelativeLocation (Variables|Default|Getcurtain1) (Math|Vector|MakeVector (.x _newtrack_3) 4.0 86.0) false false)
          (Transformation|SetRelativeLocation (Variables|Default|Getcurtain2) (Math|Vector|MakeVector (.x _newtrack_1) 4.0 86.0) false false))
        (:Finished
          (Variables|Default|Setis_finished true)
          (Variables|/Game/Blueprints/BP_GameMode.BP_GameMode_C|Setmonstertriggered (stale EventTick _asbp_game_mode) false)))
      (else
        (Variables|Default|Setis_open true)
        (Audio|PlaySoundatLocation "/Game/Sounds/348590__alienxxx__close-curtains.348590__alienxxx__close-curtains" "0, 0, 0" "0, 0, 0" 1.0 1.0 0.0 0 0 0)
        (Timeline|Timeline_1 PlayFromStart)))))

(fn ConstructionScript)