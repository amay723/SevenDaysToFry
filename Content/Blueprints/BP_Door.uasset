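; BP_Door is an interactable door that swings open or closed with a creaking sound.
; Interact toggles IsOpen and plays the DoorOpenClose timeline forward to open or in reverse to close, driving the Door component's relative yaw.
; An IsFinished flag blocks further interaction until the timeline finishes.
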(event EventBeginPlay)

(event Collision|EventActorBeginOverlap
  (params (OtherActor :type Actor%20Object%20Reference)))

(event EventTick
  (params (DeltaSeconds :type Float%20%28single-precision%29)))

(event EventInteract
  (if (Variables|Default|GetbIsFinished)
    (Variables|Default|SetbIsFinished false)
    (if (Variables|Default|GetbIsOpen)
      (Variables|Default|SetbIsOpen false)
      (Audio|PlaySoundatLocation "/Game/Sounds/458049__quetzalcontla__door-creaking.458049__quetzalcontla__door-creaking" "0, 0, 0" "0, 0, 0" 3.0 1.0 0.0 0 0 0)
      (bind _rotation (Timeline|DoorOpenClose ReverseFromEnd)
        (:Update
          (Transformation|SetRelativeRotation (Variables|Default|GetDoor) (Math|Rotator|MakeRotator 0.0 0.0 (.z _rotation)) false false))
        (:Finished
          (Variables|Default|SetbIsFinished true)))
      (else
        (Variables|Default|SetbIsOpen true)
        (Audio|PlaySoundatLocation "/Game/Sounds/458049__quetzalcontla__door-creaking.458049__quetzalcontla__door-creaking" "0, 0, 0" "0, 0, 0" 3.0 1.0 0.0 0 0 0)
        (Timeline|DoorOpenClose PlayFromStart)))))

(fn ConstructionScript)