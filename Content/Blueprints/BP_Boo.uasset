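; Boo ghost enemy, modeled on Mario's Boo, that wakes when interacted with, becoming a ghost sphere and starting the time-alive HUD once via BP_GameMode.
; Tick uses WasRecentlyRendered: unseen, it chases the player and raises Transparency_Amount; seen, it halts and lowers it, recreating the dynamic material each frame.
; Overlapping BP_Character kills it, shows the RedHit widget, records survival time in the GameMode and restarts the level after a delay.
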(event OnComponentBeginOverlap(Cube)
  (params (OverlappedComponent :type Primitive%20Component%20Object%20Reference) (OtherActor :type Actor%20Object%20Reference) (OtherComp :type Primitive%20Component%20Object%20Reference) (OtherBodyIndex :type Integer) (bFromSweep :type Boolean) (SweepResult :type Hit%20Result%20Structure%20%28by%20ref%29))
  ;[1 1 1] Death
  (bind _asbp_character (Utilities|Casting|CastToBP_Character OtherActor))
  (Default|Die _asbp_character)
  (Input|DisableInput _asbp_character 0)
  (Variables|/Game/Blueprints/BP_Character.BP_Character_C|SetCurrentSpeed _asbp_character 0.0)
  (if (Variables|Default|Gethas_hit)
    (Variables|Default|Sethas_hit false)
    (Viewport|RemoveAllWidgets)
    (bind _returnvalue (UserInterface|CreateWidget "/Game/HUD/RedHit.RedHit_C"))
    (bind _output_get (Variables|Default|SetNewVar_0 _returnvalue))
    (UserInterface|Viewport|AddtoViewport _output_get 0)
    (bind _output_get_2 (Variables|Default|Setis_dead true))
    (bind _asbp_game_mode (Utilities|Casting|CastToBP_GameMode (Game|GetGameMode)))
    (Variables|/Game/Blueprints/BP_GameMode.BP_GameMode_C|SetAlivetime _asbp_game_mode (Variables|/Game/Blueprints/BP_GameMode.BP_GameMode_C|GetTotalseconds _asbp_game_mode))
    (Variables|/Game/Blueprints/BP_GameMode.BP_GameMode_C|Setdead _asbp_game_mode _output_get_2)
    (Utilities|FlowControl|Delay 5.0)
    (Development|ExecuteConsoleCommand "Restartlevel" 0)))

(event EventBeginPlay)

(event Collision|EventActorBeginOverlap
  (params (OtherActor :type Actor%20Object%20Reference)))

(event EventTick
  (params (DeltaSeconds :type Float%20%28single-precision%29))
  (bind _returnvalue (Transformation|GetActorLocation))
  (bind _returnvalue_2 (Game|GetPlayerCharacter 0))
  (bind _returnvalue_3 (Transformation|GetActorLocation _returnvalue_2))
  (Variables|Default|SetDeltaSeconds DeltaSeconds)
  (if (Variables|Default|GetbIsActive)
    (if (Class|Actor|WasRecentlyRendered 0.2)
      (bind _output_get (Variables|Default|SetTransparencyAmount (Math|Float|Clamp(Float) (+ -0.005 (Variables|Default|GetTransparencyAmount)) 0.2)))
      (bind _returnvalue_4 (Rendering|Material|CreateDynamicMaterialInstance (Variables|Default|GetCube) 0 "/Game/MAterials/ghost1_Inst1.ghost1_Inst1" "None" :!class /Script/Engine.PrimitiveComponent))
      (bind _output_get_2 (Variables|Default|SetGhostMaterial _returnvalue_4))
      ;[1 1 1] Creation of the boo
      (Rendering|Material|SetScalarParameterValue _output_get_2 "Transparency_Amount" _output_get :!class /Script/Engine.MaterialInstanceDynamic)
      (Rendering|Material|SetMaterial (Variables|Default|GetCube) 0 (Variables|Default|GetGhostMaterial))
      (else
        (bind _output_get_3 (Variables|Default|SetTransparencyAmount (Math|Float|Clamp(Float) (+ 0.01 (Variables|Default|GetTransparencyAmount)) 0.2)))
        (bind _returnvalue_5 (Rendering|Material|CreateDynamicMaterialInstance (Variables|Default|GetCube) 0 "/Game/MAterials/ghost1_Inst1.ghost1_Inst1" "None" :!class /Script/Engine.PrimitiveComponent))
        (Variables|Default|SetGhostMaterial _returnvalue_5)
        (Rendering|Material|SetScalarParameterValue (Variables|Default|GetGhostMaterial) "Transparency_Amount" _output_get_3 :!class /Script/Engine.MaterialInstanceDynamic)
        (Rendering|Material|SetMaterial (Variables|Default|GetCube) 0 (Variables|Default|GetGhostMaterial))
        (Variables|Default|Setcount 2e+02)
        (Transformation|SetActorLocationAndRotation (+ _returnvalue (* (Math|Vector|GetUnitDirection(Vector) _returnvalue _returnvalue_3) (* (Variables|Default|GetDeltaSeconds) (Variables|Default|Getcount)))) (Math|Rotator|FindLookatRotation _returnvalue _returnvalue_3))))))

(event EventInteract
  ;[1 1 1] Creation of the boo
  (Development|PrintString "Boo Clicked")
  (Components|StaticMesh|SetStaticMesh (Variables|Default|GetCube) "/Engine/BasicShapes/Sphere.Sphere")
  (Rendering|Material|SetMaterial (Variables|Default|GetCube) 0 "/Game/MAterials/ghost1_Inst1.ghost1_Inst1")
  (Variables|Default|SetbIsActive true)
  (bind _asbp_game_mode (Utilities|Casting|CastToBP_GameMode (Game|GetGameMode)))
  (if (not (Variables|/Game/Blueprints/BP_GameMode.BP_GameMode_C|Getboo_alive _asbp_game_mode))
    (bind _returnvalue (UserInterface|CreateWidget "/Game/HUD/InGameHUD.InGameHUD_C"))
    (bind _output_get (Variables|Default|SetTimeAliveHuD _returnvalue))
    (UserInterface|Viewport|AddtoViewport _output_get 1)
    (Variables|/Game/Blueprints/BP_GameMode.BP_GameMode_C|Setboo_alive _asbp_game_mode true)))

(fn ConstructionScript)