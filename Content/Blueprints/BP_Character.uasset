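; BP_Character is the first-person player character, using gaze-and-touch controls to move and interact.
; Each tick traces from the camera for interface-implementing actors; touch sends InteractMessage to the gazed actor, otherwise moves along camera forward while held.
; Mouse axes steer the view, and BeginPlay adds a BestTime widget.
; Die plays a one-time sound and sets a flag that Tick uses to run a camera-roll timeline, which clears it when finished.
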(event Custom|GazeCheck
  (bind _camera (Variables|Default|GetCamera))
  (bind _returnvalue (Transformation|GetWorldLocation _camera))
  ;[1 1 1] Gaze check
  (bind _outhit (Collision|LineTraceByChannel _returnvalue (+ _returnvalue (* (Math|Vector|GetForwardVector _camera) 2000)) "TraceTypeQuery1" false 0 "ForOneFrame"))
  (if (Utilities|DoesObjectImplementInterface (.HitActor (Collision|BreakHitResult _outhit)) "/Game/Blueprints/BP_Interactive_Interface.BP_Interactive_Interface_C")
    (Variables|Default|SetInteractive_Actor (.HitActor (Collision|BreakHitResult _outhit)))
    (else
      (Variables|Default|SetInteractive_Actor 0))))

(event EventBeginPlay
  (Variables|Default|SetI_AM_DEAD false)
  (bind _returnvalue (UserInterface|CreateWidget "/Game/HUD/BestTime.BestTime_C"))
  (bind _output_get (Variables|Default|SetNewVar_4 _returnvalue))
  (UserInterface|Viewport|AddtoViewport _output_get 1))

(event EventTick
  (params (DeltaSeconds :type Float%20%28single-precision%29))
  ;[1 1 1] Tick
  (CallFunction|GazeCheck)
  (Class|PawnMovementComponent|AddInputVector (Variables|Character|GetCharacterMovement) (* (* (Math|Vector|GetForwardVector (Variables|Default|GetCamera)) (Variables|Default|GetCurrentSpeed)) DeltaSeconds) false)
  (if (Variables|Default|GetI_AM_DEAD)
    (bind _newtrack_1 (Timeline|Deathrattle Play)
      (:Update
        (Transformation|SetRelativeRotation (Variables|Default|GetCamera) (Math|Rotator|MakeRotator (.x _newtrack_1) 0.0 0.0) false false))
      (:Finished
        (Variables|Default|SetI_AM_DEAD false)))))

(event Input|ActionEvents|InputActionTouch
  (params (Key :type Key%20Structure))
  (bind _interactive_actor (Variables|Default|GetInteractive_Actor))
  ;[1 1 1] Input
  (:Pressed
    (Utilities|IsValid _interactive_actor
      (:Is%20Valid
        (Class|BPInteractiveInterface|Interact(Message) _interactive_actor))
      (:Is%20Not%20Valid
        (Variables|Default|SetCurrentSpeed 1e+02))))
  (:Released
    (Variables|Default|SetCurrentSpeed 0.0)))

(event Input|AxisEvents|InputAxismouseX
  (params (AxisValue :type Float%20%28single-precision%29))
  ;[1 1 1] Input
  (Pawn|Input|AddControllerYawInput AxisValue))

(event Input|AxisEvents|InputAxismouseY
  (params (AxisValue :type Float%20%28single-precision%29))
  ;[1 1 1] Input
  (Pawn|Input|AddControllerPitchInput AxisValue))

(fn ConstructionScript)

(fn Die
  (if (not (Variables|Default|GetI_AM_DEAD))
    (Variables|Default|SetI_AM_DEAD true)
    (if (not (Variables|Default|GetSound_Played))
      (Audio|PlaySoundatLocation "/Game/Sounds/173126__replix__death-sound-male.173126__replix__death-sound-male" "0, 0, 0" "0, 0, 0" 5.0 1.0 0.2 0 0 0)
      (Variables|Default|SetSound_Played true))))