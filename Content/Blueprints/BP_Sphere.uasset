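; BP_Sphere is an interactable actor that switches its particle system on and off.
; Each Interact event prints a "Sphere Clicked" message, flips the ParticleActive flag and activates or deactivates the particle system to match.
; The construction script feeds the same flag into the particle system's auto-activate setting, so its value sets the starting state.
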(event EventBeginPlay)

(event Collision|EventActorBeginOverlap
  (params (OtherActor :type Actor%20Object%20Reference)))

(event EventTick
  (params (DeltaSeconds :type Float%20%28single-precision%29)))

(event EventInteract
  (bind _particlesystem (Variables|Default|GetParticleSystem))
  (Development|PrintString "Sphere Clicked")
  (if (Variables|Default|GetbParticleActive)
    (Variables|Default|SetbParticleActive false)
    (Components|Activation|Deactivate _particlesystem)
    (else
      (Variables|Default|SetbParticleActive true)
      (Components|Activation|Activate _particlesystem false))))

(fn ConstructionScript
  (Components|Activation|SetAutoActivate (Variables|Default|GetParticleSystem) (Variables|Default|GetbParticleActive)))