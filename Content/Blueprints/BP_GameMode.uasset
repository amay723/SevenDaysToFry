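; BP_GameMode is a game mode that tracks play time and the player's best survival time.
; While BooAlive is set, Tick adds delta time to Totalseconds.
; If Dead is also set, it copies Alivetime into MyGameInstance's BestTime unless the stored value is greater.
; Disconnected SaveGame chains for persisting the best time to a slot never run, so this graph saves nothing to disk.
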(event EventBeginPlay)

(event EventTick
  (params (DeltaSeconds :type Float%20%28single-precision%29))
  (bind _alivetime (Variables|Default|GetAlivetime))
  (if (Variables|Default|Getboo_alive)
    (bind _output_get (Variables|Default|Setseconds DeltaSeconds))
    (Variables|Default|Settotalseconds (+ (Variables|Default|Gettotalseconds) _output_get))
    (if (Variables|Default|Getdead)
      (bind _asmy_game_instance (Utilities|Casting|CastToMyGameInstance (Game|GetGameInstance)))
      (if (not (> (Variables|/Game/MyGameInstance.MyGameInstance_C|GetBestTime _asmy_game_instance) _alivetime))
        (Variables|/Game/MyGameInstance.MyGameInstance_C|SetBestTime _asmy_game_instance _alivetime)))))

(fn ConstructionScript)