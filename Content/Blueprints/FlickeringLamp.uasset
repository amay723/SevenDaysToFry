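; A flickering lamp actor whose point light blinks until an interaction breaks it.
; Tick runs chained Delays, 0.4 seconds then StopFlickering, before toggling the light's visibility, and the construction script starts it visible.
; Interact works once, hiding the light, playing a sound at its location and setting StopFlickering to a huge value so later Delays effectively never finish, instead of gating Tick on Broken.
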(event EventBeginPlay)

(event Collision|EventActorBeginOverlap
  (params (OtherActor :type Actor%20Object%20Reference)))

(event EventTick
  (params (DeltaSeconds :type Float%20%28single-precision%29))
  (Utilities|FlowControl|Delay 0.4)
  (Utilities|FlowControl|Delay (stale EventInteract _output_get))
  (Rendering|ToggleVisibility (Variables|Default|GetPointLight) false))

(event EventInteract
  (if (not (Variables|Default|GetBroken))
    (Rendering|SetVisibility (Variables|Default|GetPointLight) false false)
    (bind _output_get (Variables|Default|SetStopFlickering 1e+09))
    (Variables|Default|SetBroken true)
    (Audio|PlaySoundatLocation "/Engine/EditorSounds/Notifications/CompileFailed.CompileFailed" (Transformation|GetWorldLocation (Variables|Default|GetPointLight)) "0, 0, 0" 1.0 1.0 0.0 0 0 0)))

(fn ConstructionScript
  (Rendering|SetVisibility (Variables|Default|GetPointLight) true false))