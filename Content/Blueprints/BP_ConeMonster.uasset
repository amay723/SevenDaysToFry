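; BP_ConeMonster is an enemy that periodically hunts the player and kills on contact.
; While the game mode's BooAlive is set, Tick starts the hunt when elapsed whole seconds divide by 15, then moves it straight toward the player with sound.
; Interact returns it to its start and ends the hunt.
; Cone overlap kills the character, shows a red hit widget, records survival time, then restarts the level after a delay.
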(event OnComponentBeginOverlap(Cone)
  (params (OverlappedComponent :type Primitive%20Component%20Object%20Reference) (OtherActor :type Actor%20Object%20Reference) (OtherComp :type Primitive%20Component%20Object%20Reference) (OtherBodyIndex :type Integer) (bFromSweep :type Boolean) (SweepResult :type Hit%20Result%20Structure%20%28by%20ref%29))
  ;[1 1 1] Death
  (bind _asbp_character (Utilities|Casting|CastToBP_Character OtherActor))
  (Default|Die _asbp_character)
  (Input|DisableInput _asbp_character 0)
  (Variables|/Game/Blueprints/BP_Character.BP_Character_C|SetCurrentSpeed _asbp_character 0.0)
  (if (Variables|Default|GetHas_hit)
    (Variables|Default|SetHas_hit false)
    (Viewport|RemoveAllWidgets)
    (bind _returnvalue (UserInterface|CreateWidget "/Game/HUD/RedHit.RedHit_C"))
    (bind _output_get (Variables|Default|SetNewVar_0 _returnvalue))
    (UserInterface|Viewport|AddtoViewport _output_get 0)
    (bind _output_get_2 (Variables|Default|Setis_dead true))
    (bind _asbp_game_mode (Utilities|Casting|CastToBP_GameMode (Game|GetGameMode)))
    (Variables|/Game/Blueprints/BP_GameMode.BP_GameMode_C|SetAlivetime _asbp_game_mode (Variables|/Game/Blueprints/BP_GameMode.BP_GameMode_C|GetTotalseconds _asbp_game_mode))
    (Variables|/Game/Blueprints/BP_GameMode.BP_GameMode_C|Setdead _asbp_game_mode _output_get_2)
    (Utilities|FlowControl|Delay 5.0)
    (Development|ExecuteConsoleCommand "Restartlevel" 0)))

(event Collision|EventActorBeginOverlap
  (params (OtherActor :type Actor%20Object%20Reference)))

(event EventTick
  (params (DeltaSeconds :type Float%20%28single-precision%29))
  (bind _returnvalue (Transformation|GetActorLocation))
  (bind _asbp_game_mode (Utilities|Casting|CastToBP_GameMode (Game|GetGameMode)))
  (Development|PrintString (Utilities|String|ToString(Integer) (Variables|Default|Getactivation_time)))
  (Variables|Default|SetDeltaSeconds DeltaSeconds)
  (Variables|Default|Setactivation_time (Math|Float|Truncate (Variables|/Game/Blueprints/BP_GameMode.BP_GameMode_C|GetTotalseconds _asbp_game_mode)))
  (if (Variables|/Game/Blueprints/BP_GameMode.BP_GameMode_C|Getboo_alive _asbp_game_mode)
    (Utilities|FlowControl|Delay 0.0)
    (if (== (Math|Integer|%(Integer) (Variables|Default|Getactivation_time) 15) 0)
      (Variables|/Game/Blueprints/BP_GameMode.BP_GameMode_C|Setmonstertriggered _asbp_game_mode true)
      (Variables|Default|SetHunting true)
      (elif (Variables|Default|GetHunting)
        (Transformation|SetActorLocation (+ _returnvalue (* (Math|Vector|GetUnitDirection(Vector) _returnvalue (Transformation|GetActorLocation (Game|GetPlayerCharacter 0))) (* (Variables|Default|GetDeltaSeconds) 2.5e+02))) false false)
        (Audio|PlaySoundatLocation (Variables|Default|Getsound) (+ _returnvalue (* (Math|Vector|GetUnitDirection(Vector) _returnvalue (Transformation|GetActorLocation (Game|GetPlayerCharacter 0))) (* (Variables|Default|GetDeltaSeconds) 2.5e+02))) "0, 0, 0" 0.3 0.5 3.3 0 0 0)))))

(event EventBeginPlay
  (Variables|Default|Setstarterlocation (Transformation|GetWorldLocation (Variables|Default|GetCone))))

(event EventInteract
  (Transformation|SetActorLocation (Variables|Default|Getstarterlocation) false false)
  (Variables|Default|SetHunting false))

(fn ConstructionScript)