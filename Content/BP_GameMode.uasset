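; Game mode that runs the cash economy, upgrade purchases and wave counter, and creates the HUD and gain/loss popups.
; Purchases read costs from CommerceData rows and pass BalanceCheck before deducting Balance.
; They respawn a destroyed barricade, swap the gun actor for the next tier (FifthUpgrade is empty), or shorten GrillTime.
; Tick increments WaveCount when GameTime crosses a high threshold, using WaveCheck as a latch reset at a low one.
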(event EventBeginPlay
  (bind _returnvalue (UserInterface|CreateWidget "/Game/HUD/Main_HUD.Main_HUD_C"))
  (bind _output_get (Variables|Default|SetMain_HUD _returnvalue))
  (UserInterface|Viewport|AddtoViewport _output_get 0)
  (bind _returnvalue_2 (UserInterface|CreateWidget "/Game/GainCash.GainCash_C"))
  (bind _output_get_2 (Variables|Default|SetGainCash _returnvalue_2))
  (UserInterface|Viewport|AddtoViewport _output_get_2 0)
  (Widget|SetVisibility _output_get_2 "Hidden")
  (bind _returnvalue_3 (UserInterface|CreateWidget "/Game/LoseCash.LoseCash_C"))
  (bind _output_get_3 (Variables|Default|SetLoseCash _returnvalue_3))
  (UserInterface|Viewport|AddtoViewport _output_get_3 0)
  (Widget|SetVisibility _output_get_3 "Hidden")
  (bind _returnvalue_4 (Utilities|GetDataTableRow "/Game/CommerceData.CommerceData" "2")
    (:then
      (Variables|Default|SetCurrentGunUPrice (.cost (Utilities|Struct|BreakCommerceStruct _returnvalue_4)))
      (bind _returnvalue_5 (Utilities|GetDataTableRow "/Game/CommerceData.CommerceData" "7")
        (:then
          (Variables|Default|SetCurrentGrillUPrice (.cost (Utilities|Struct|BreakCommerceStruct _returnvalue_5)))
          (bind _output_get_4 (Variables|Default|Setguns%20transform (Math|Transform|MakeTransform "-268.000000,763.000000,308.000000" "0,-90.000000, 0" "1,1,1")))
          (bind _returnvalue_6 (Game|SpawnActorfromClass "/Game/gun.gun_C" _output_get_4 "Undefined" 0 0))
          (Variables|Default|Setgun _returnvalue_6))))))

(event EventTick
  (params (DeltaSeconds :type Float%20%28single-precision%29))
  (Utilities|FlowControl|Sequence
    (:then_0
      ;[1 1 1] Wave Set and Checks
      (if (Variables|Default|GetWaveCheck)
        (if (<= (Variables|Default|GetGameTime) 1e+02)
          (Variables|Default|SetWaveCheck false))
        (elif (>= (Variables|Default|GetGameTime) 8e+02)
          (Variables|Default|SetWaveCount (+ (Variables|Default|GetWaveCount) 1))
          (Variables|Default|SetWaveCheck true))))))

(fn ConstructionScript)

(fn RecreateBarricade
  (if (Variables|Default|GetBarricadeDestroyed)
    (bind _returnvalue (Utilities|GetDataTableRow "/Game/CommerceData.CommerceData" "1")
      (:then
        (bind (_is_balance_positive_ _newbalance) (CallFunction|BalanceCheck (.cost (Utilities|Struct|BreakCommerceStruct _returnvalue))))
        (if _is_balance_positive_
          (CallFunction|NegativeCashFlow (.cost (Utilities|Struct|BreakCommerceStruct _returnvalue)))
          (Variables|Default|SetBalance _newbalance)
          (Game|SpawnActorfromClass "/Game/BreakingBarricade.BreakingBarricade_C" (Variables|Default|GetBarricadeTransform) "Undefined" 0 0)
          (Variables|Default|SetBarricadeDestroyed false)
          (CallFunction|VanishWidget false)
          (else
            (Development|PrintString "YOUR BROKE")))))))

(fn BalanceCheck
  (params (Price :type Float%20%28single-precision%29))
  (bind _balance (Variables|Default|GetBalance))
  (bind _returnvalue (- _balance Price))
  (if (>= _returnvalue 0.0)
    (return true _returnvalue)))

(fn FirstUpgrade
  (bind _returnvalue (Utilities|GetDataTableRow "/Game/CommerceData.CommerceData" "2")
    (:then
      (bind (_is_balance_positive_ _newbalance) (CallFunction|BalanceCheck (.cost (Utilities|Struct|BreakCommerceStruct _returnvalue))))
      (if _is_balance_positive_
        (CallFunction|NegativeCashFlow (.cost (Utilities|Struct|BreakCommerceStruct _returnvalue)))
        (Variables|Default|SetBalance _newbalance)
        (Actor|DestroyActor (Variables|Default|Getgun))
        (bind _returnvalue_2 (Game|SpawnActorfromClass "/Game/gun2.gun2_C" (Variables|Default|Getguns%20transform) "Undefined" 0 0))
        (Variables|Default|Setgun2 _returnvalue_2)
        (bind _returnvalue_3 (Utilities|GetDataTableRow "/Game/CommerceData.CommerceData" "3")
          (:then
            (Variables|Default|SetCurrentGunUPrice (.cost (Utilities|Struct|BreakCommerceStruct _returnvalue_3)))
            (CallFunction|VanishWidget false)))
        (else
          (Development|PrintString "YOUR BROKE"))))))

(fn SecondUpgrade
  (bind _returnvalue (Utilities|GetDataTableRow "/Game/CommerceData.CommerceData" "3")
    (:then
      (bind (_is_balance_positive_ _newbalance) (CallFunction|BalanceCheck (.cost (Utilities|Struct|BreakCommerceStruct _returnvalue))))
      (if _is_balance_positive_
        (CallFunction|NegativeCashFlow (.cost (Utilities|Struct|BreakCommerceStruct _returnvalue)))
        (Variables|Default|SetBalance _newbalance)
        (Actor|DestroyActor (Variables|Default|Getgun2))
        (bind _returnvalue_2 (Game|SpawnActorfromClass "/Game/gun3.gun3_C" (Variables|Default|Getguns%20transform) "Undefined" 0 0))
        (Variables|Default|Setgun3 _returnvalue_2)
        (bind _returnvalue_3 (Utilities|GetDataTableRow "/Game/CommerceData.CommerceData" "4")
          (:then
            (Variables|Default|SetCurrentGunUPrice (.cost (Utilities|Struct|BreakCommerceStruct _returnvalue_3)))
            (CallFunction|VanishWidget false)))
        (else
          (Development|PrintString "YOUR BROKE"))))))

(fn ThirdUpgrade
  (bind _returnvalue (Utilities|GetDataTableRow "/Game/CommerceData.CommerceData" "4")
    (:then
      (bind (_is_balance_positive_ _newbalance) (CallFunction|BalanceCheck (.cost (Utilities|Struct|BreakCommerceStruct _returnvalue))))
      (if _is_balance_positive_
        (CallFunction|NegativeCashFlow (.cost (Utilities|Struct|BreakCommerceStruct _returnvalue)))
        (Variables|Default|SetBalance _newbalance)
        (Actor|DestroyActor (Variables|Default|Getgun3))
        (bind _returnvalue_2 (Game|SpawnActorfromClass "/Game/gun4.gun4_C" (Variables|Default|Getguns%20transform) "Undefined" 0 0))
        (Variables|Default|Setgun4 _returnvalue_2)
        (bind _returnvalue_3 (Utilities|GetDataTableRow "/Game/CommerceData.CommerceData" "10")
          (:then
            (Variables|Default|SetCurrentGunUPrice (.cost (Utilities|Struct|BreakCommerceStruct _returnvalue_3)))
            (CallFunction|VanishWidget false)))
        (else
          (Development|PrintString "YOUR BROKE"))))))

(fn FourthUpgrade
  (bind _returnvalue (Utilities|GetDataTableRow "/Game/CommerceData.CommerceData" "5")
    (:then
      (bind (_is_balance_positive_ _newbalance) (CallFunction|BalanceCheck (.cost (Utilities|Struct|BreakCommerceStruct _returnvalue))))
      (if _is_balance_positive_
        (CallFunction|NegativeCashFlow (.cost (Utilities|Struct|BreakCommerceStruct _returnvalue)))
        (Variables|Default|SetBalance _newbalance)
        (Actor|DestroyActor (Variables|Default|Getgun4))
        (bind _returnvalue_2 (Game|SpawnActorfromClass "/Game/gun5.gun5_C" (Variables|Default|Getguns%20transform) "Undefined" 0 0))
        (Variables|Default|Setgun5 _returnvalue_2)
        (CallFunction|VanishWidget false)
        (else
          (Development|PrintString "YOUR BROKE"))))))

(fn FifthUpgrade)

(fn GrillUpgrade
  (switch int (Variables|Default|GetGrillUCount)
    (:0
      (bind _returnvalue (Utilities|GetDataTableRow "/Game/CommerceData.CommerceData" "7")
        (:then
          (bind (_is_balance_positive_ _newbalance) (CallFunction|BalanceCheck (.cost (Utilities|Struct|BreakCommerceStruct _returnvalue))))
          (if _is_balance_positive_
            (CallFunction|NegativeCashFlow (.cost (Utilities|Struct|BreakCommerceStruct _returnvalue)))
            (Variables|Default|SetBalance _newbalance)
            (Variables|Default|SetGrillTime (- (Variables|Default|GetGrillTime) 2.0))
            (Variables|Default|SetGrillUCount (+ (Variables|Default|GetGrillUCount) 1))
            (bind _returnvalue_2 (Utilities|GetDataTableRow "/Game/CommerceData.CommerceData" "8")
              (:then
                (Variables|Default|SetCurrentGrillUPrice (.cost (Utilities|Struct|BreakCommerceStruct _returnvalue_2)))
                (CallFunction|VanishWidget false)))
            (else
              (Development|PrintString "YOUR BROKE"))))))
    (:1
      (bind _returnvalue_3 (Utilities|GetDataTableRow "/Game/CommerceData.CommerceData" "8")
        (:then
          (bind (_is_balance_positive__2 _newbalance_2) (CallFunction|BalanceCheck (.cost (Utilities|Struct|BreakCommerceStruct _returnvalue_3))))
          (if _is_balance_positive__2
            (CallFunction|NegativeCashFlow (.cost (Utilities|Struct|BreakCommerceStruct _returnvalue_3)))
            (Variables|Default|SetBalance _newbalance_2)
            (Variables|Default|SetGrillTime (- (Variables|Default|GetGrillTime) 2.0))
            (Variables|Default|SetGrillUCount (+ (Variables|Default|GetGrillUCount) 1))
            (bind _returnvalue_4 (Utilities|GetDataTableRow "/Game/CommerceData.CommerceData" "9")
              (:then
                (Variables|Default|SetCurrentGrillUPrice (.cost (Utilities|Struct|BreakCommerceStruct _returnvalue_4)))
                (CallFunction|VanishWidget false)))
            (else
              (Development|PrintString "YOUR BROKE"))))))
    (:2
      (bind _returnvalue_5 (Utilities|GetDataTableRow "/Game/CommerceData.CommerceData" "9")
        (:then
          (bind (_is_balance_positive__3 _newbalance_3) (CallFunction|BalanceCheck (.cost (Utilities|Struct|BreakCommerceStruct _returnvalue_5))))
          (if _is_balance_positive__3
            (CallFunction|NegativeCashFlow (.cost (Utilities|Struct|BreakCommerceStruct _returnvalue_5)))
            (Variables|Default|SetBalance _newbalance_3)
            (Variables|Default|SetGrillTime (- (Variables|Default|GetGrillTime) 2.0))
            (Variables|Default|SetGrillUCount (+ (Variables|Default|GetGrillUCount) 1))
            (bind _returnvalue_6 (Utilities|GetDataTableRow "/Game/CommerceData.CommerceData" "10")
              (:then
                (Variables|Default|SetCurrentGrillUPrice (.cost (Utilities|Struct|BreakCommerceStruct _returnvalue_6)))
                (CallFunction|VanishWidget false)))
            (else
              (Development|PrintString "YOUR BROKE"))))))))

(fn PositiveCashFlow
  (params (PositiveCash :type Float%20%28single-precision%29))
  (Variables|Default|SetPositiveCash PositiveCash)
  (Widget|SetVisibility (Variables|Default|GetGainCash) "Visible")
  (Audio|SpawnSoundAttached "/Game/Sounds/MoneySound.MoneySound" (Variables|/Script/Engine.Character|GetMesh (Variables|Default|GetCurrentCustomer)) "None" "0, 0, 0" "0, 0, 0" "KeepRelativeOffset" false 1.0 1.0 0.0 0 0))

(fn VanishWidget
  (params (gain :type Boolean))
  (if gain
    (Widget|SetVisibility (Variables|Default|GetGainCash) "Hidden")
    (else
      (Widget|SetVisibility (Variables|Default|GetLoseCash) "Hidden"))))

(fn NegativeCashFlow
  (params (cost :type Float%20%28single-precision%29))
  (Variables|Default|SetNegativeCash cost)
  (Widget|SetVisibility (Variables|Default|GetLoseCash) "Visible"))